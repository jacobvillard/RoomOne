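; Bomb actor with a timed fuse that explodes and shatters into physics debris.
; LightFuse runs a timeline scaled to the fuse time, dissolving the animated fuse's material and sliding sparks between its sockets.
; On completion it fires a Niagara explosion preloaded with a sim cache, then shortly swaps the mesh for a Geometry Collection broken by strain field and radial impulse.
; Chaos removal events count down pieces to set the actor's lifespan.
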(event OnChaosRemovalEvent(BombGC)
  (params (RemovalEvent :type Chaos%20Removal%20Event%20Structure%20%28by%20ref%29))
  (bind _output_get (Variables|Default|SetPiecesCount (- (Variables|Default|GetPiecesCount) 1)))
  (if (< _output_get 1)
    (Actor|SetLifeSpan 2.0)))

(event Custom|LightFuse
  (params (FuseTimer :type Float%20%28double-precision%29))
  (bind _fuse (Variables|Default|GetFuse))
  (bind _returnvalue (Transformation|GetSocketTransform _fuse "FuseEnd" "RTS_World"))
  (Components|Timeline|SetPlayRate (Variables|Default|GetFuseTimeline) (/ 1.0 FuseTimer))
  (Components|Activation|Activate (Variables|Default|GetNS_FuseSparks) false)
  (Components|Animation|PlayAnimation (Variables|Default|GetFuse) "/Game/CustomMeshes/Bomb/FuseAnim.FuseAnim" true)
  (bind (_direction _burnamount _sparkposition) (Timeline|FuseTimeline Play)
    (:Update
      (Rendering|Material|SetScalarParameterValue (Variables|Default|GetFuseDMI) "DissolveAmount" _burnamount :!class /Script/Engine.MaterialInstanceDynamic)
      (Utilities|FlowControl|Sequence
        (:then_0
          (Transformation|SetWorldLocation (Variables|Default|GetNS_FuseSparks) (Math|Vector|Lerp(Vector) (.location _returnvalue) (.location (Transformation|GetSocketTransform (Variables|Default|GetFuse) "FuseBase" "RTS_World")) _sparkposition) false false))
        (:then_1
          (Transformation|SetWorldRotation (Variables|Default|GetNS_FuseSparks) (Math|Rotator|Lerp(Rotator) (.rotation _returnvalue) "0.000000,1.000000,0.000000" _sparkposition) false false))))
    (:Finished
      (Components|Activation|Deactivate (Variables|Default|GetNS_FuseSparks))
      (Utilities|Time|SetTimerbyEvent (delegate Custom|BreakBomb) 0.4)
      (Components|Activation|Activate (Variables|Default|GetBombExplosion) false)
      (Collision|SetCollisionEnabled (Variables|Default|GetStaticMesh) "NoCollision"))))

(event Custom|BreakBomb
  (bind _bombgc (Variables|Default|GetBombGC))
  (Rendering|SetVisibility (Variables|Default|GetStaticMesh) false false)
  (Rendering|SetVisibility (Variables|Default|GetBombGC) true false)
  (Physics|SetSimulatePhysics (Variables|Default|GetBombGC) true)
  (bind _returnvalue (AddComponent|AddRadialFalloff))
  (Class|FieldSystemComponent|ApplyPhysicsField (Variables|Default|GetFieldSystem) true "Field_ExternalClusterStrain" 0 (Field|SetRadialFalloff _returnvalue 5e+05 0.0 1.0 0.0 2e+02 (Transformation|GetWorldLocation (Variables|Default|GetBombGC)) "Field_FallOff_None"))
  (Physics|AddRadialImpulse _bombgc (- (Transformation|GetWorldLocation _bombgc) "0.000000,0.000000,100.000000") 2e+02 1.5e+04 "RIF_Constant" false))

(event EventBeginPlay
  (|CallParentFunction)
  (Class|NiagaraComponent|SetSimCache (Variables|Default|GetBombExplosion) "/Game/CustomMeshes/Bomb/NS_BombExplosion_SimCache_ExplosionCache.NS_BombExplosion_SimCache_ExplosionCache" false)
  (Variables|Default|SetPiecesCount (Utilities|Array|Length (Components|GetChildrenComponents (Variables|Default|GetBombGC) true))))

(fn ConstructionScript
  (|CallParentFunction)
  (bind _returnvalue (Rendering|Material|CreateDynamicMaterialInstance (Variables|Default|GetFuse) 0 "/Game/CustomMeshes/Bomb/FuseMat.FuseMat" "None" :!class /Script/Engine.PrimitiveComponent))
  (Variables|Default|SetFuseDMI _returnvalue))