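; BP_ClientLaptop is an interactable laptop that players focus on to use a WBP_LeaveBTN widget, created on BeginPlay.
; Sphere overlap shows a camera-facing key hint and binds the character's InteractEvent; leaving hides it and unbinds.
; Interacting toggles focus, switching the view target between laptop and character, along with input mode, cursor, hint visibility and movement through server calls.
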(event OnComponentBeginOverlap(Sphere)
  (params (OverlappedComponent :type Primitive%20Component%20Object%20Reference) (OtherActor :type Actor%20Object%20Reference) (OtherComp :type Primitive%20Component%20Object%20Reference) (OtherBodyIndex :type Integer) (bFromSweep :type Boolean) (SweepResult :type Hit%20Result%20Structure%20%28by%20ref%29))
  ;[0.2462 0.6038 1] Widget Key Hint
  (bind _asbp_third_person_character (Utilities|Casting|CastToBP_ThirdPersonCharacter OtherActor))
  (if (Pawn|IsLocalPlayerController (Game|GetPlayerController 0))
    (bind _asbp_third_person_character_2 (Utilities|Casting|CastToBP_ThirdPersonCharacter (Game|GetPlayerCharacter 0)))
    (CallFunction|ClientToggleWidget false)
    (EventDispatchers|BindEventtoInteractEvent _asbp_third_person_character (delegate Custom|RadioInterfactEvent))))

(event OnComponentEndOverlap(Sphere)
  (params (OverlappedComponent :type Primitive%20Component%20Object%20Reference) (OtherActor :type Actor%20Object%20Reference) (OtherComp :type Primitive%20Component%20Object%20Reference) (OtherBodyIndex :type Integer))
  ;[0.2462 0.6038 1] Widget Key Hint
  (bind _asbp_third_person_character (Utilities|Casting|CastToBP_ThirdPersonCharacter OtherActor))
  (if (Pawn|IsLocalPlayerController (Game|GetPlayerController 0))
    (CallFunction|ClientToggleWidget true)
    (if (Utilities|IsValid _asbp_third_person_character)
      (EventDispatchers|UnbindallEventsfromInteractEvent _asbp_third_person_character))))

(event Custom|Client%20ToggleWidget
  (params (Hide :type Boolean))
  ;[0.2462 0.6038 1] Widget Key Hint
  (CallFunction|FuncToggleWidget (Variables|Default|GetWidget1) Hide))

(event Custom|RadioInterfactEvent
  (params (Host :type Boolean))
  ;[0.2462 0.6038 1] Widget Key Hint
  ;;[1 0.1176 0.9569] Interact with Device
  (CallFunction|FuncInteractwithDevices))

(event EventBeginPlay
  (bind _returnvalue (Game|GetPlayerCharacter 0))
  ;[0.2462 0.6038 1] Widget Key Hint
  (if (Pawn|IsLocallyControlled _returnvalue)
    (Development|PrintString (Utilities|GetDisplayName _returnvalue))
    (bind _returnvalue_2 (UserInterface|CreateWidget "/Game/UserInterface/WBP_LeaveBTN.WBP_LeaveBTN_C" (Game|GetPlayerController 0)))
    (UserInterface|SetWidget (Variables|Default|GetWidget2) _returnvalue_2)
    (Variables|Default|SetWidgetLeaveLobby _returnvalue_2)
    (CallFunction|ClientToggleWidget true)
    (if (Utilities|IsValid (stale OnComponentEndOverlap(Sphere) _asbp_third_person_character))
      (EventDispatchers|UnbindallEventsfromInteractEvent (stale OnComponentEndOverlap(Sphere) _asbp_third_person_character)))))

(event Collision|EventActorBeginOverlap
  (params (OtherActor :type Actor%20Object%20Reference)))

(event EventTick
  (params (DeltaSeconds :type Float%20%28single-precision%29))
  (bind _widget1 (Variables|Default|GetWidget1))
  ;[0.2462 0.6038 1] Widget Key Hint
  (if (and (Variables|Default|GetPlayerInSphere) (Utilities|IsValid (stale OnComponentBeginOverlap(Sphere) _asbp_third_person_character)))
    (Transformation|SetWorldRotation _widget1 (Math|Rotator|FindLookatRotation (Transformation|GetWorldLocation _widget1) (Transformation|GetWorldLocation (Variables|/Script/RoomOne.RoomOneCharacter|GetFollowCamera (stale OnComponentBeginOverlap(Sphere) _asbp_third_person_character_2)))) false false)))

(fn ConstructionScript)

(fn FuncToggleWidget
  (params (Scene%20Comp :type Scene%20Component%20Object%20Reference) (hide :type Boolean))
  (Development|SetHiddeninGame Scene%20Comp hide false)
  (Variables|Default|SetPlayerInSphere (== hide false)))

(fn FuncInteractwithDevices
  (bind _returnvalue (Game|GetPlayerCharacter 0))
  (bind _returnvalue_2 (Game|GetPlayerController 0))
  (bind _widget1 (Variables|Default|GetWidget1))
  ;[1 0.1176 0.9569] Interact with Device
  (if (Variables|Default|GetisFocused)
    (Game|Player|SetViewTargetwithBlend _returnvalue_2 _returnvalue 0.0 "VTBlend_Linear" 0.0 false)
    (Input|SetInputModeGameOnly _returnvalue_2 false)
    (Variables|/Script/Engine.PlayerController|SetbShowMouseCursor _returnvalue_2 false)
    (bind _asbp_third_person_character (Utilities|Casting|CastToBP_ThirdPersonCharacter _returnvalue)
      (:then
        (Default|ServerRenableMovement _asbp_third_person_character))
      (:CastFailed
        _))
    (Development|SetHiddeninGame _widget1 false false)
    (Variables|Default|SetisFocused false)
    (UserInterface|CreateWidget "/Game/UserInterface/WBP_LeaveBTN.WBP_LeaveBTN_C")
    (else
      (Game|Player|SetViewTargetwithBlend _returnvalue_2 self 0.0 "VTBlend_Linear" 0.0 false) ; Set Camera Target
      (Input|SetInputModeGameandUI _returnvalue_2 0 "DoNotLock" false false) ; Çhangine input mode
      (Variables|/Script/Engine.PlayerController|SetbShowMouseCursor _returnvalue_2 true) ; Update cursor visibility
      (bind _asbp_third_person_character_2 (Utilities|Casting|CastToBP_ThirdPersonCharacter _returnvalue)
        (:then
          (Default|ServerDisableMovement _asbp_third_person_character_2))
        (:CastFailed
          _))
      (Development|SetHiddeninGame _widget1 true false) ; Set the widget visibility
      (Variables|Default|SetisFocused true)
      (bind _aswdp_key_hint_1 (Utilities|Casting|CastToWDP_KeyHint1 (UserInterface|GetWidget _widget1)))
      (Default|UpdateKey _aswdp_key_hint_1))))