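; BP_GetChained is an interactable actor with a proximity key hint; its chaining logic is unfinished.
; Sphere overlaps with any third-person character toggle the hint widget when player controller 0 is local, and Tick turns it toward that character's follow camera while shown.
; Host and client interact events only print and cache all player characters.
; BeginPlay hides the hint and creates, but never displays, a leave-button widget.
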(event OnComponentBeginOverlap(Sphere)
  (params (OverlappedComponent :type Primitive%20Component%20Object%20Reference) (OtherActor :type Actor%20Object%20Reference) (OtherComp :type Primitive%20Component%20Object%20Reference) (OtherBodyIndex :type Integer) (bFromSweep :type Boolean) (SweepResult :type Hit%20Result%20Structure%20%28by%20ref%29))
  ;[0.2462 0.6038 1] Widget Key Hint
  (bind _asbp_third_person_character (Utilities|Casting|CastToBP_ThirdPersonCharacter OtherActor))
  (if (Pawn|IsLocalPlayerController (Game|GetPlayerController 0))
    (CallFunction|ClientToggleWidget false)))

(event OnComponentEndOverlap(Sphere)
  (params (OverlappedComponent :type Primitive%20Component%20Object%20Reference) (OtherActor :type Actor%20Object%20Reference) (OtherComp :type Primitive%20Component%20Object%20Reference) (OtherBodyIndex :type Integer))
  ;[0.2462 0.6038 1] Widget Key Hint
  (Utilities|Casting|CastToBP_ThirdPersonCharacter OtherActor)
  (if (Pawn|IsLocalPlayerController (Game|GetPlayerController 0))
    (CallFunction|ClientToggleWidget true)))

(event Custom|Client%20ToggleWidget
  (params (Hide :type Boolean))
  ;[0.2462 0.6038 1] Widget Key Hint
  (CallFunction|FuncToggleWidget (Variables|Default|GetWidget1) Hide))

(event EventBeginPlay
  ;[0.2462 0.6038 1] Widget Key Hint
  (bind _returnvalue (UserInterface|CreateWidget "/Game/UserInterface/WBP_LeaveBTN.WBP_LeaveBTN_C"))
  (Variables|Default|SetWidgetLeaveLobby _returnvalue)
  (CallFunction|ClientToggleWidget true))

(event Collision|EventActorBeginOverlap
  (params (OtherActor :type Actor%20Object%20Reference)))

(event EventTick
  (params (DeltaSeconds :type Float%20%28single-precision%29))
  (bind _widget1 (Variables|Default|GetWidget1))
  ;[0.2462 0.6038 1] Widget Key Hint
  (if (Variables|Default|GetPlayerInSphere)
    (Transformation|SetWorldRotation _widget1 (Math|Rotator|FindLookatRotation (Transformation|GetWorldLocation _widget1) (Transformation|GetWorldLocation (Variables|/Script/RoomOne.RoomOneCharacter|GetFollowCamera (stale OnComponentBeginOverlap(Sphere) _asbp_third_person_character)))) false false)))

(event EventHostInteractEvent
  ;[1 0.1176 0.9569] Get Chained
  (Development|PrintString "Host")
  (bind _outactors (Actor|GetAllActorsOfClass "/Game/ThirdPerson/Blueprints/BP_ThirdPersonCharacter.BP_ThirdPersonCharacter_C"))
  (Variables|Default|SetPlayerCharacters _outactors))

(event EventClientInteractEvent
  ;[1 0.1176 0.9569] Get Chained
  (Development|PrintString "Client")
  (bind _outactors (Actor|GetAllActorsOfClass "/Game/ThirdPerson/Blueprints/BP_ThirdPersonCharacter.BP_ThirdPersonCharacter_C"))
  (Variables|Default|SetPlayerCharacters _outactors))

(fn ConstructionScript)

(fn FuncToggleWidget
  (params (Scene%20Comp :type Scene%20Component%20Object%20Reference) (hide :type Boolean))
  (Development|SetHiddeninGame Scene%20Comp hide false)
  (Variables|Default|SetPlayerInSphere (== hide false)))