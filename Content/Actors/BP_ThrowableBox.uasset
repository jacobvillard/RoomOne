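; Throwable box actor that players can pick up and drop, and that ragdolls characters overlapping its box trigger while it is not held.
; A sphere trigger shows a key hint to the local player, rotated each tick toward their follow camera.
; Pickup and drop reset rotation and relay held state through server-to-client events, with a delay on drop to prevent self-ragdoll.
; Similar replicated events toggle mesh collision.
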(event OnComponentBeginOverlap(Box)
  (params (OverlappedComponent :type Primitive%20Component%20Object%20Reference) (OtherActor :type Actor%20Object%20Reference) (OtherComp :type Primitive%20Component%20Object%20Reference) (OtherBodyIndex :type Integer) (bFromSweep :type Boolean) (SweepResult :type Hit%20Result%20Structure%20%28by%20ref%29))
  ;[1 0.1176 0.9569] Trigger Ragdoll
  (bind _asbp_third_person_character (Utilities|Casting|CastToBP_ThirdPersonCharacter OtherActor))
  (if (not (Variables|Default|GetHeld)) ; If the player is not already holding this box
    (Default|TriggerRagdoll _asbp_third_person_character) ; Ragdoll player
  ))

(event OnComponentBeginOverlap(Sphere)
  (params (OverlappedComponent :type Primitive%20Component%20Object%20Reference) (OtherActor :type Actor%20Object%20Reference) (OtherComp :type Primitive%20Component%20Object%20Reference) (OtherBodyIndex :type Integer) (bFromSweep :type Boolean) (SweepResult :type Hit%20Result%20Structure%20%28by%20ref%29))
  ;[0.5333 0.8 1] Widget Handling
  ;;[0.5333 0.8 1] Enable  Widget
  (bind (_locallycontrolled _asbp_third_person_character) (CallFunction|FuncEnableWidget OtherActor (Variables|Default|GetWidget))))

(event OnComponentEndOverlap(Sphere)
  (params (OverlappedComponent :type Primitive%20Component%20Object%20Reference) (OtherActor :type Actor%20Object%20Reference) (OtherComp :type Primitive%20Component%20Object%20Reference) (OtherBodyIndex :type Integer))
  ;[0.5333 0.8 1] Widget Handling
  ;;[0.5333 0.8 1] Disable Widget
  (CallFunction|FuncDisableWidget (Variables|Default|GetWidget) OtherActor))

(event Custom|Server%20Update%20Collision
  (params (collisionDisabled :type Boolean))
  (CallFunction|RPCUpdateCollision collisionDisabled))

(event Custom|Dropped
  ;[0 1 0] State Updates
  (Transformation|SetActorRotation "0, 0, 0") ; Reset actor rotation to keep hint on top
  (Utilities|FlowControl|Delay 0.2) ; Grace Period to prevent self ragdoll
  (CallFunction|FuncUpdateHeldState false) ; Updates the held state
)

(event Custom|PickedUp
  ;[0 1 0] State Updates
  (CallFunction|FuncUpdateHeldState true) ; Updates the held state
  (Development|SetHiddeninGame (Variables|Default|GetWidget) true false) ; Hides key hint when held
  (Utilities|FlowControl|Delay 0.15)
  (Transformation|SetActorRotation "0, 0, 0") ; Reset actor rotation to keep hint on top
)

(event Custom|RPC%20UpdateCollision
  (params (NewParam :type Boolean))
  (bind _staticmesh (Variables|Default|GetStaticMesh))
  (if NewParam
    (Collision|SetCollisionEnabled _staticmesh "NoCollision")
    (else
      (Collision|SetCollisionEnabled _staticmesh "QueryAndPhysics"))))

(event Custom|Server%20InformServerOfHeldState
  (params (Held :type Boolean))
  ;[0 1 0] State Updates
  ;;[1 0.3647 0] Network Replication
  (CallFunction|RPCInformClientsOfHeldState Held))

(event Custom|RPC%20InformClientsOfHeldState
  (params (Held :type Boolean))
  ;[0 1 0] State Updates
  ;;[1 0.3647 0] Network Replication
  (Variables|Default|SetHeld Held))

(event EventBeginPlay
  ;[0.5333 0.8 1] Hide Key Hint On Begin Play
  (Development|SetHiddeninGame (Variables|Default|GetWidget) true false))

(event EventTick
  (params (DeltaSeconds :type Float%20%28single-precision%29))
  ;[0.5333 0.8 1] Widget Handling
  ;;[0.5333 0.8 1] Ensure Widget Always Faces Camera
  (CallFunction|FuncUpdateWIdgetRotation (stale OnComponentBeginOverlap(Sphere) _locallycontrolled) (stale OnComponentBeginOverlap(Sphere) _asbp_third_person_character) (Variables|Default|GetWidget)))

(fn ConstructionScript)

(fn FuncUpdateHeldState
  (params (Held :type Boolean))
  (bind _output_get (Variables|Default|SetHeld Held))
  (CallFunction|ServerInformServerOfHeldState _output_get))

(fn FuncDisableWidget
  (params (W_KeyHint :type Scene%20Component%20Object%20Reference) (OtherActor :type Actor%20Object%20Reference))
  (bind _asbp_third_person_character (Utilities|Casting|CastToBP_ThirdPersonCharacter OtherActor))
  (if (Pawn|IsLocallyControlled _asbp_third_person_character)
    (Development|SetHiddeninGame W_KeyHint true false) ; Hides key hint when out of range
    (Variables|Default|SetPlayerInSphere false) ; Update flag
  ))

(fn FuncEnableWidget
  (params (OtherActor :type Actor%20Object%20Reference) (Widget :type Scene%20Component%20Object%20Reference))
  (bind _asbp_third_person_character (Utilities|Casting|CastToBP_ThirdPersonCharacter OtherActor))
  (if (Pawn|IsLocallyControlled _asbp_third_person_character)
    (bind _asbp_third_person_character_2 (Utilities|Casting|CastToBP_ThirdPersonCharacter (Game|GetPlayerCharacter 0)))
    (if (not (Variables|Default|GetHeld))
      (Development|SetHiddeninGame Widget false false) ; Shows key hint when in range
      (Variables|Default|SetPlayerInSphere true) ; Update flag
      (return (Pawn|IsLocallyControlled _asbp_third_person_character) _asbp_third_person_character_2))))

(fn FuncUpdateWIdgetRotation
  (params (LocallyControlled :type Boolean) (Player :type Room%20One%20Character%20Object%20Reference) (Widget :type Scene%20Component%20Object%20Reference))
  (if (Math|Boolean|ANDBoolean (Variables|Default|GetPlayerInSphere) LocallyControlled (Utilities|IsValid Player)) ; Only run if player is in sphere and locally controlled
    (Transformation|SetWorldRotation (Variables|Default|GetWidget) (Math|Rotator|FindLookatRotation (Transformation|GetWorldLocation Widget) (Transformation|GetWorldLocation (Variables|/Script/RoomOne.RoomOneCharacter|GetFollowCamera Player))) false false)))