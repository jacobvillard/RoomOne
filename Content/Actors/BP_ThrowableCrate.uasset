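; BP_ThrowableCrate is a crate actor that shatters when it hits something hard enough.
; Static mesh hit events compare the normal impulse magnitude against ImpulseThreshold.
; Past the threshold, a DoOnce spawns a BP_BreakableCrate at the same transform, passes it the flipped, damped impulse, then destroys the original crate.
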(event OnComponentHit(StaticMesh)
  (params (HitComponent :type Primitive%20Component%20Object%20Reference) (OtherActor :type Actor%20Object%20Reference) (OtherComp :type Primitive%20Component%20Object%20Reference) (NormalImpulse :type Vector :default "0, 0, 0") (Hit :type Hit%20Result%20Structure%20%28by%20ref%29))
  ;[0.15 0.15 0.15 0.5] Spawn Breakable Box on Hit if impact force is greater than ImpulseThreshold
  (Variables|Default|SetNormal%20Impulse NormalImpulse)
  (if (> (Math|Vector|VectorLength (Variables|Default|GetNormal%20Impulse)) (Variables|Default|GetImpulseThreshold))
    (Utilities|FlowControl|DoOnce false ; Stops Multiple Boxes Spawning
      (:Completed
        ;;[0.15 0.15 0.15 0.5] Spawn Breakable Box and Apply Impulse
        (bind _returnvalue (Game|SpawnActorfromClass "/Game/Actors/BP_BreakableCrate.BP_BreakableCrate_C" (Transformation|GetActorTransform) "AlwaysSpawn" "MultiplyWithRoot" 0 0))
        (Default|Impulse _returnvalue (/ (* (Variables|Default|GetNormal%20Impulse) -1.0) (Variables|Default|GetVelocityDamper)))
        (Actor|DestroyActor) ; Destroy Thrown Box
      ))))

(event EventBeginPlay
  (|CallParentFunction))

(event Collision|EventActorBeginOverlap
  (params (OtherActor :type Actor%20Object%20Reference)))

(event EventTick
  (params (DeltaSeconds :type Float%20%28single-precision%29))
  (|CallParentFunction DeltaSeconds) ; This node is disabled and will not be called.\nDrag off pins to build functionality.
)

(fn ConstructionScript
  (|CallParentFunction))