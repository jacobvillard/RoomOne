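; BP_DoorWayCode2 is a Ball Run actor that randomizes a binary trap code for each of its Doors and displays it on gems.
; On authority, SetDoorCode rolls each code, passes it to the door's SetTrap and forwards it with the index through ServSetCode to RPCSetCode.
; RPCSetCode colors the matching gem green or pink and prints the code for debugging.
; The construction script gathers the three gem components into an array.
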(event Custom|Serv%20set%20code
  (params (Int :type Integer) (Index :type Integer))
  (CallFunction|RPCSetCode Int Index))

(event Custom|SetDoorCode
  (Networking|SwitchHasAuthority
    (:Authority
      (for (_array_element _array_index) (Variables|Default|Get%20Doors)
        (bind _output_get (Variables|Default|SetCurrentCode (Math|Random|RandomIntegerinRange 0 1)))
        (Default|SetTrap _array_element _output_get)
        (CallFunction|ServSetCode _output_get _array_index)))))

(event Custom|RPC%20SetCode
  (params (Int :type Integer) (Index :type Integer))
  (bind _gems (Variables|Default|GetGems))
  (bind _output (Utilities|Array|Get(acopy) _gems Index))
  (Development|PrintString (Utilities|String|Append "Code" (Utilities|String|ToString(Integer) Int)) true true "(R=0.000000,G=0.660000,B=1.000000,A=1.000000)" 1e+02)
  (switch int Int
    (:0
      (Rendering|Material|SetMaterial _output 0 "/Game/ThirdPerson/AlexiAssets/GemGreen.GemGreen"))
    (:1
      (Rendering|Material|SetMaterial _output 0 "/Game/ThirdPerson/AlexiAssets/GemPink.GemPink"))))

(fn ConstructionScript
  (Variables|Default|SetGems (Utilities|Array|MakeArray (Variables|Default|GetGem0) (Variables|Default|GetGem1) (Variables|Default|GetGem2))))