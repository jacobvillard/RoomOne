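; BP_CaveFinish is a finish-zone actor that ends the roped-together cave level and returns the session to the lobby.
; Its box tracks overlapping third-person characters, and each entry reads the player count from the game instance and enables Tick.
; Tick waits until the overlap count strictly exceeds that number, then starts a one-time delay before a console ServerTravel to LobbyMap as a listen server.
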(event OnComponentBeginOverlap(Box)
  (params (OverlappedComponent :type Primitive%20Component%20Object%20Reference) (OtherActor :type Actor%20Object%20Reference) (OtherComp :type Primitive%20Component%20Object%20Reference) (OtherBodyIndex :type Integer) (bFromSweep :type Boolean) (SweepResult :type Hit%20Result%20Structure%20%28by%20ref%29))
  (bind _asbp_third_person_character (Utilities|Casting|CastToBP_ThirdPersonCharacter OtherActor))
  (Utilities|Array|Add (Variables|Default|GetOverlappingPlayers) _asbp_third_person_character)
  (bind _asgame_instance_bp (Utilities|Casting|CastToGameInstanceBP (Game|GetGameInstance)))
  (Variables|Default|SetNumPlayers (Variables|/Game/GameInstanceBP.GameInstanceBP_C|GetNumOfPlayers _asgame_instance_bp))
  (Actor|Tick|SetActorTickEnabled true))

(event OnComponentEndOverlap(Box)
  (params (OverlappedComponent :type Primitive%20Component%20Object%20Reference) (OtherActor :type Actor%20Object%20Reference) (OtherComp :type Primitive%20Component%20Object%20Reference) (OtherBodyIndex :type Integer))
  (bind _asbp_third_person_character (Utilities|Casting|CastToBP_ThirdPersonCharacter OtherActor))
  (Utilities|Array|RemoveItem (Variables|Default|GetOverlappingPlayers) _asbp_third_person_character))

(event Custom|CustomEvent)

(event Custom|EndGame
  (Development|ExecuteConsoleCommand "ServerTravel  /Game/ThirdPerson/Maps/LobbyMap?listen" 0))

(event EventBeginPlay)

(event EventTick
  (params (DeltaSeconds :type Float%20%28single-precision%29))
  (if (> (Utilities|Array|Length (Variables|Default|GetOverlappingPlayers)) (Variables|Default|GetNumPlayers))
    (if (not (Variables|Default|GetFinished))
      (Variables|Default|SetFinished true)
      (Utilities|Time|SetTimerbyEvent (delegate Custom|EndGame) 8.0))))

(fn ConstructionScript)