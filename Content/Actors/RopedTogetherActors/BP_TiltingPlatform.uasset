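; BP_TiltingPlatform is a roped-together obstacle whose mesh rocks back and forth in pitch between positive and negative TiltAngle.
; BeginPlay scales a timeline's play rate by TimeForFullSwing and starts it, with each timeline update lerping the mesh's relative rotation.
; On finish, the Go event calls itself with the direction flipped to alternate Play and Reverse.
; The Activate event is empty, and its RopeActivator binding is disconnected.
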(event Custom|Activate)

(event Custom|Go!
  (params (Forward :type Boolean))
  (bind _tiltangle (Variables|Settings|GetTiltAngle))
  (if Forward
    (bind _alpha (Timeline|TiltingPlatform Play)
      (:Update
        (Transformation|SetRelativeRotation (Variables|Default|GetStaticMesh) (Math|Rotator|Lerp(Rotator) (Math|Rotator|MakeRotator 0.0 _tiltangle 0.0) (Math|Rotator|MakeRotator 0.0 (* _tiltangle -1.0) 0.0) _alpha) false true))
      (:Finished
        (CallFunction|Go! (not Forward))))
    (else
      (Timeline|TiltingPlatform Reverse))))

(event EventBeginPlay
  (Components|Timeline|SetPlayRate (Variables|Default|GetTiltingPlatform) (/ 1.0 (Variables|Settings|GetTimeForFullSwing)))
  (CallFunction|Go! true))

(fn ConstructionScript)