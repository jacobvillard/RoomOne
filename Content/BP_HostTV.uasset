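; BP_HostTV is an interactable TV actor that switches the local player into a focused view of itself.
; A sphere overlap shows a prompt widget only for a locally controlled player with authority, and Tick turns it toward that character's follow camera.
; InteractEvent flip-flops between the TV view with cursor, UI input, disabled movement and hidden prompt, and normal third-person play.
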(event OnComponentBeginOverlap(Sphere)
  (params (OverlappedComponent :type Primitive%20Component%20Object%20Reference) (OtherActor :type Actor%20Object%20Reference) (OtherComp :type Primitive%20Component%20Object%20Reference) (OtherBodyIndex :type Integer) (bFromSweep :type Boolean) (SweepResult :type Hit%20Result%20Structure%20%28by%20ref%29))
  (bind _asbp_third_person_character (Utilities|Casting|CastToBP_ThirdPersonCharacter OtherActor))
  (if (and (Pawn|IsLocallyControlled (Game|GetPlayerCharacter 0)) (Ability|HasAuthority (Game|GetPlayerController 0)))
    (Development|SetHiddeninGame (Variables|Default|GetWidget1) false false)
    (Variables|Default|SetPlayerInSphere true)))

(event OnComponentEndOverlap(Sphere)
  (params (OverlappedComponent :type Primitive%20Component%20Object%20Reference) (OtherActor :type Actor%20Object%20Reference) (OtherComp :type Primitive%20Component%20Object%20Reference) (OtherBodyIndex :type Integer))
  (Utilities|Casting|CastToBP_ThirdPersonCharacter OtherActor)
  (if (and (Pawn|IsLocallyControlled (Game|GetPlayerCharacter 0)) (Ability|HasAuthority (Game|GetPlayerController 0)))
    (Development|SetHiddeninGame (Variables|Default|GetWidget1) true false)
    (Variables|Default|SetPlayerInSphere false)))

(event EventBeginPlay
  (Development|SetHiddeninGame (Variables|Default|GetWidget1) true false)
  (Variables|Default|SetPlayerInSphere false))

(event Collision|EventActorBeginOverlap
  (params (OtherActor :type Actor%20Object%20Reference)))

(event EventTick
  (params (DeltaSeconds :type Float%20%28single-precision%29))
  (bind _widget1 (Variables|Default|GetWidget1))
  (if (Variables|Default|GetPlayerInSphere)
    (Transformation|SetWorldRotation _widget1 (Math|Rotator|FindLookatRotation (Transformation|GetWorldLocation _widget1) (Transformation|GetWorldLocation (Variables|/Script/RoomOne.RoomOneCharacter|GetFollowCamera (stale OnComponentBeginOverlap(Sphere) _asbp_third_person_character)))) false false)))

(event EventInteractEvent
  (bind _returnvalue (Game|GetPlayerCharacter 0))
  (bind _returnvalue_2 (Game|GetPlayerController 0))
  (bind _widget1 (Variables|Default|GetWidget1))
  (bind _charactermovement (Variables|/Script/Engine.Character|GetCharacterMovement _returnvalue))
  (Utilities|FlowControl|FlipFlop
    (:A
      (Game|Player|SetViewTargetwithBlend _returnvalue_2 self 0.0 "VTBlend_Linear" 0.0 false)
      (Input|SetInputModeGameandUI _returnvalue_2 0 "DoNotLock" false false)
      (Variables|/Script/Engine.PlayerController|SetbShowMouseCursor _returnvalue_2 true)
      (Pawn|Components|CharacterMovement|DisableMovement _charactermovement)
      (Development|SetHiddeninGame _widget1 true false))
    (:B
      (Game|Player|SetViewTargetwithBlend _returnvalue_2 _returnvalue 0.0 "VTBlend_Linear" 0.0 false)
      (Input|SetInputModeGameOnly _returnvalue_2 false)
      (Variables|/Script/Engine.PlayerController|SetbShowMouseCursor _returnvalue_2 false)
      (Pawn|Components|CharacterMovement|SetMovementMode _charactermovement "MOVE_Walking" 0)
      (Development|SetHiddeninGame _widget1 false false))))

(fn ConstructionScript)