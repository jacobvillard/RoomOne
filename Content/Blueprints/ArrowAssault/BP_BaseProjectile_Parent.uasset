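; Parent projectile for ArrowAssault that damages the player on hit, and damages enemies only after being deflected by a shield.
; Speed and gravity apply in the construction script, and the spawner's collision is briefly ignored on BeginPlay.
; Each hit broadcasts OnProjectileContact, then branches by cast: shields enable bouncing, other hits destroy the projectile.
; Impacts spawn a visual effect and a sound that varies through an ImpactType integer parameter.
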(event OnComponentHit(BoxCollision)
  (params (HitComponent :type Primitive%20Component%20Object%20Reference) (OtherActor :type Actor%20Object%20Reference) (OtherComp :type Primitive%20Component%20Object%20Reference) (NormalImpulse :type Vector :default "0, 0, 0") (Hit :type Hit%20Result%20Structure%20%28by%20ref%29))
  (bind (_bblockinghit _binitialoverlap _time _distance _location _impactpoint _normal _impactnormal _physmat _hitactor) (Collision|BreakHitResult Hit))
  ;[0.15 0.15 0.15 0.5] When the projectile collider hits another collider, does effect(s), applies damage and destroys the actor. Different behaviour and Impact Sound depending on what was hit. Impact Type Key: 0 = Hit Immune/Nothing, 1 = Hit Immune, 2 = Hit Shield, 3 = Hit Character
  (Default|CallOnProjectileContact OtherActor Hit)
  (Utilities|Casting|CastToBP_Shield _hitactor ; If Shield hit, it deflects
    (:then
      (Variables|Default|SetDeflected true)
      (Variables|/Script/Engine.ProjectileMovementComponent|SetbShouldBounce (Variables|Default|GetProjectileMovement) true)
      (Variables|Default|SetImpactType 2) ; Hit Shield
      (CallFunction|ImpactFX _location)
      (Variables|Default|SetImpactType 3) ; Will Hit Character (Enemy)
    )
    (:CastFailed
      (Utilities|Casting|CastToBP_Enemy _hitactor ; If Enemy hit...
        (:then
          (if (Variables|Default|GetDeflected) ; Checks if deflected
            (CallFunction|DamageActor _hitactor) ; Only damage if deflected
            (CallFunction|ImpactFX _location) ; Plays FX
            (Actor|DestroyActor)
            (else
              (Variables|Default|SetImpactType 1) ; Hit Immune
              (CallFunction|ImpactFX _location)
              (Actor|DestroyActor))))
        (:CastFailed
          (Utilities|Casting|CastToBP_ThirdPersonCharacter _hitactor ; If Player hit...
            (:then
              (Variables|Default|SetImpactType 3) ; Hit Character (Player)
              (CallFunction|DamageActor _hitactor) ; Damage Player
              (CallFunction|ImpactFX _location)
              (Actor|DestroyActor))
            (:CastFailed
              (Variables|Default|SetImpactType 0) ; Hit Nothing
              (CallFunction|ImpactFX _location)
              (Actor|DestroyActor))))))))

(event Custom|ImpactFX
  (params (Location :type Vector))
  ;[0.15 0.15 0.15 0.5] Plays Visual and Audiual effect and then destroys the Projectile
  (Niagara|SpawnSystematLocation (Variables|Effects|GetImpact%20Visual) Location)
  (bind _returnvalue (Audio|SpawnSoundatLocation (Variables|Effects|GetImpact%20Sound) Location "0, 0, 0" 1.0 1.0 0.0 0 0))
  (Effects|Components|ParticleSystem|SetIntParameter _returnvalue "ImpactType" (Variables|Default|GetImpactType)))

(event Custom|DamageActor
  (params (Damaged%20Actor :type Actor%20Object%20Reference))
  ;[0.15 0.15 0.15 0.5] Applies damage to the hit actor
  (Game|Damage|ApplyDamage Damaged%20Actor (Variables|ProjectileSettings|GetProjectileDmg) 0 0)
  (Utilities|FlowControl|Delay 3.0)
  (Actor|DestroyActor))

(event EventBeginPlay
  (bind _returnvalue (Components|GetOwner))
  ;[0.15 0.15 0.15 0.5] On Spawn (Play) Temporarily ignores the collider of the spawner
  (Collision|IgnoreActorwhenMoving (Variables|Default|GetBoxCollision) _returnvalue true)
  (Utilities|FlowControl|Delay 0.1)
  (Collision|IgnoreActorwhenMoving (Variables|Default|GetBoxCollision) _returnvalue false))

(fn ConstructionScript
  (bind _projectilemovement (Variables|Default|GetProjectileMovement))
  (bind _speed (Variables|ProjectileSettings|GetSpeed))
  ;[0.15 0.15 0.15 0.5] Allows for editing individual projectiles in spawn actor if needed
  (Variables|/Script/Engine.ProjectileMovementComponent|SetInitialSpeed _projectilemovement _speed)
  (Variables|/Script/Engine.ProjectileMovementComponent|SetMaxSpeed _projectilemovement _speed)
  (Variables|/Script/Engine.ProjectileMovementComponent|SetProjectileGravityScale _projectilemovement (Variables|ProjectileSettings|GetGravity)))