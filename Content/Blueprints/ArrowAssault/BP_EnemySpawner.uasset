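; Spawns a grid formation of BP_Enemy actors at BeginPlay, each set to fire arrow projectiles with targeting enabled.
; Row and column counts left at zero are randomized within small ranges before spawning.
; Nested loops offset from the spawner along world X and Y, tracing a short ray down the actor's up axis at each cell.
; Enemies spawn raised above the hit point, only where that trace hits.
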(event EventBeginPlay
  ;[0.15 0.15 0.15 0.5] Chooses Random Formation and Spawns Enemies in Grid
  (CallFunction|GetRandomRows)
  (CallFunction|GetRandomCols)
  (CallFunction|GridSpawnActors))

(fn ConstructionScript)

(fn GridSpawnActors
  (bind _returnvalue (Transformation|GetActorLocation))
  (bind _returnvalue_2 (Transformation|GetActorLocation))
  ;[0.15 0.15 0.15 0.5] Uses rays to form the X axis of the grid spawner . Red Arrow in Viewport reveals which direction it will spawn the objects
  (for _index (range 0 (- (Variables|EnemyGrid|GetEnemiesCols) 1)) ; Last Index = Number of Rows
    (Collision|LineTraceByChannel (Math|Vector|MakeVector (+ (* _index 1000) (.x _returnvalue)) (.y _returnvalue) (.z _returnvalue)) (+ (Math|Vector|MakeVector (+ (* _index 1000) (.x _returnvalue)) (.y _returnvalue) (.z _returnvalue)) (* (Math|Vector|GetUpVector (Transformation|GetActorRotation)) -1e+01)) "TraceTypeQuery1" false 0 "None") ; Cast Ray. Use Draw Debug Type to see casts
    ;[0.15 0.15 0.15 0.5] Using rays, and the X axis of the rays before, forms the Y axis of the grid spawner.
    (for _index_2 (range 0 (- (Variables|EnemyGrid|GetEnemiesRows) 1)) ; Last Index = Number of Rows
      (bind (_outhit _returnvalue_3) (Collision|LineTraceByChannel (Math|Vector|MakeVector (+ (* _index 1000) (.x _returnvalue)) (+ (* _index_2 400) (.y _returnvalue_2)) (.z _returnvalue_2)) (+ (Math|Vector|MakeVector (+ (* _index 1000) (.x _returnvalue)) (+ (* _index_2 400) (.y _returnvalue_2)) (.z _returnvalue_2)) (* (Math|Vector|GetUpVector (Transformation|GetActorRotation)) -1e+01)) "TraceTypeQuery1" false 0 "None")) ; Cast Ray. Use Draw Debug Type to see casts
      ;[0.15 0.15 0.15 0.5] (X Axis) If Ray hit, Spawn Enemy at Ray Location
      (if _returnvalue_3
        (Game|SpawnActorfromClass "/Game/Blueprints/ArrowAssault/BP_Enemy.BP_Enemy_C" (Math|Transform|MakeTransform (+ (.Location (Collision|BreakHitResult _outhit)) "0.000000,0.000000,180.000000") "0.000000,180.000000,0.000000" "1.000000,1.000000,1.000000") "Undefined" "MultiplyWithRoot" 0 4.0 "/Game/Blueprints/ArrowAssault/BP_BaseProjectile_Child_Arrow.BP_BaseProjectile_Child_Arrow_C" true 1.0 0)))))

(fn GetRandomRows
  ;[0.15 0.15 0.15 0.5] Generates a random formation from range if rows is set to 0
  (if (== (Variables|EnemyGrid|GetEnemiesRows) 0)
    (Variables|EnemyGrid|SetEnemiesRows (Math|Random|RandomIntegerinRange 1 5))))

(fn GetRandomCols
  ;[0.15 0.15 0.15 0.5] Generates a random formation from range if columns is set to 0
  (if (== (Variables|EnemyGrid|GetEnemiesCols) 0)
    (Variables|EnemyGrid|SetEnemiesCols (Math|Random|RandomIntegerinRange 1 6))))