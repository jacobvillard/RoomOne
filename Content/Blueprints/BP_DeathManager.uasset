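; BP_DeathManager is a trigger actor that respawns any BP_ThirdPersonCharacter overlapping it.
; At BeginPlay it gathers spawn points from the actors attached to a SpawnPointsParent actor.
; On overlap, authority only, it waits briefly, picks the spawn point nearest the character's overlap location, and calls ServerTeleportToRespawn with that transform.
; A ragdoll call is present but disconnected, and a message prints when no spawn points exist.
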(event EventBeginPlay
  (Variables|Default|SetSpawnPoints (Actor|GetAttachedActors (Variables|Default|GetSpawnPointsParent) true false)))

(event Collision|EventActorBeginOverlap
  (params (OtherActor :type Actor%20Object%20Reference))
  (bind _spawnpoints (Variables|Default|GetSpawnPoints))
  (Networking|SwitchHasAuthority
    (:Authority
      (bind _asbp_third_person_character (Utilities|Casting|CastToBP_ThirdPersonCharacter OtherActor))
      (Variables|Default|SetPlayerLoc (Transformation|GetActorLocation _asbp_third_person_character))
      (if (> (Utilities|Array|Length _spawnpoints) 0)
        (Utilities|FlowControl|Delay 0.5)
        (for (_array_element _array_index) _spawnpoints
          (if (== _array_index 0)
            (Variables|Default|SetClosestDistance (Math|Vector|Distance(Vector) (Variables|Default|GetPlayerLoc) (Transformation|GetActorLocation _array_element)))
            (Variables|Default|SetClosestLocation (Transformation|GetActorTransform _array_element) :!label _label)
            (elif (< (Math|Vector|Distance(Vector) (Variables|Default|GetPlayerLoc) (Transformation|GetActorLocation _array_element)) (Variables|Default|GetClosestDistance))
              (Variables|Default|SetClosestDistance (Math|Vector|Distance(Vector) (Variables|Default|GetPlayerLoc) (Transformation|GetActorLocation _array_element)))
              (goto _label))))
        (Default|ServerTeleporttoRespawn _asbp_third_person_character (Variables|Default|GetClosestLocation))
        (else
          (Development|PrintString "There are no spawn points configured"))))))

(event EventTick
  (params (DeltaSeconds :type Float%20%28single-precision%29)))

(fn ConstructionScript)