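; Hero character that walks to a chest on its own, damages it, then destroys itself.
; On BeginPlay the authority sets walk speed, finds a BP_Chest and, after a short delay, runs AI MoveTo toward it.
; Success triggers the chest's TakeDamage and removes the hero, while failure only prints debug strings.
; The construction script assigns a random skeletal mesh from the Meshes list.
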(event EventBeginPlay
  (Networking|SwitchHasAuthority
    (:Authority
      (Variables|/Script/Engine.CharacterMovementComponent|SetMaxWalkSpeed (Variables|Character|GetCharacterMovement) (Variables|Default|GetWalkSpeed))
      (bind _returnvalue (Actor|GetActorOfClass "/Game/Blueprints/BP_Chest.BP_Chest_C"))
      (Utilities|FlowControl|Delay 0.1)
      (bind _movementresult (AI|AIMoveTo self "4200.000000,3330.000000,142.012604" _returnvalue 1.5e+02 false)
        (:OnSuccess
          (Development|PrintString "success?")
          (Default|TakeDamage _returnvalue)
          (Actor|DestroyActor))
        (:OnFail
          (Development|PrintString (Utilities|String|EnumtoString _movementresult))
          (Development|PrintString "Hello"))))))

(fn ConstructionScript
  (Components|SkeletalMesh|SetSkeletalMeshAsset (Variables|Character|GetMesh) (.OutItem (Utilities|Array|Random (Variables|Default|GetMeshes)))))