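; BP_MinecartActor is a minecart that moves continuously along its right vector at a set Speed.
; On BeginPlay it stores its starting transform and starts a looping timer on ResetInterval.
; Each timer firing teleports it back to the start, so the motion repeats as a loop without any track or spline.
; Tick applies the frame-scaled world offset without sweeping for collision.
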(event Custom|Reset
  (Transformation|SetActorTransform self (stale EventBeginPlay _output_get) false true))

(event EventBeginPlay
  (bind _output_get (Variables|Default|SetStartTransform (Transformation|GetActorTransform self)))
  (Utilities|Time|SetTimerbyEvent (delegate Custom|Reset) (Variables|Default|GetResetInterval) true))

(event Collision|EventActorBeginOverlap
  (params (OtherActor :type Actor%20Object%20Reference)))

(event EventTick
  (params (DeltaSeconds :type Float%20%28single-precision%29))
  (Transformation|AddActorWorldOffset self (* (Transformation|GetActorRightVector) (* DeltaSeconds (Variables|Default|GetSpeed)))))

(fn ConstructionScript)