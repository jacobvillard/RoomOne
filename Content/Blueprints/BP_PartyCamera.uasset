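; BP_PartyCamera is a shared camera that follows and frames all BP_ThirdPersonCharacter players.
; A looping timer averages their positions into a target at a fixed height, ignoring jumps and falls.
; It also records the farthest player's distance from the previous target.
; Once a target exists, Tick smoothly moves the actor there and maps that radius to spring arm length for zoom.
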(event Custom|RecalculateCameraTargets
  (Variables|Default|SetVectorPosition "0, 0, 0") ; Reset var
  (Variables|Default|SetRaduis 0.0)
  (bind _outactors (Actor|GetAllActorsOfClass "/Game/Blueprints/Characters/Goblin/BP_ThirdPersonCharacter.BP_ThirdPersonCharacter_C")) ; Get all players
  ;[0.15 0.15 0.15 0.5] Calculate center of all players
  (for _array_element _outactors
    (Variables|Default|SetVectorPosition (+ (Transformation|GetActorLocation _array_element) (Variables|Default|GetVectorPosition)))
    (if (and (> (Math|Vector|Distance(Vector) (Transformation|GetActorLocation _array_element) (stale _output_get_2)) (Variables|Default|GetRaduis)) (Utilities|HasTargetLocationInitialized))
      (bind _output_get (Variables|Default|SetRaduis (Math|Vector|Distance(Vector) (Transformation|GetActorLocation _array_element) (stale _output_get_2))))))
  (bind _output_get_2 (Variables|Default|SetTargetLocation (Math|Vector|MakeVector (.X (Math|Vector|BreakVector (/ (Variables|Default|GetVectorPosition) (Utilities|Array|Length _outactors)))) (.Y (Math|Vector|BreakVector (/ (Variables|Default|GetVectorPosition) (Utilities|Array|Length _outactors)))) (Variables|Default|GetZ))))
  (Variables|Default|SetMaxRadius _output_get))

(event EventBeginPlay
  (Utilities|Time|SetTimerbyEvent (delegate Custom|RecalculateCameraTargets) (Variables|Default|GetUpdateRate) true true))

(event EventTick
  (params (DeltaSeconds :type Float%20%28single-precision%29))
  (bind _springarm (Variables|Default|GetSpringArm))
  (if (Utilities|HasTargetLocationInitialized) ; Only once target location is set
    (Transformation|SetActorLocation (Math|Interpolation|VInterpTo (Transformation|GetActorLocation) (Variables|Default|GetTargetLocation) DeltaSeconds (Variables|Default|GetFollowSpeed)) false false)
    (Variables|/Script/Engine.SpringArmComponent|SetTargetArmLength _springarm (Math|Interpolation|FInterpTo (Variables|/Script/Engine.SpringArmComponent|GetTargetArmLength _springarm) (Math|Float|MapRangeClamped (Variables|Default|GetMaxRadius) 2e+02 2e+03 (Variables|Default|GetMinTargetArmLength) (Variables|Default|GetMaxTargetArmLength)) DeltaSeconds (Variables|Default|GetZoomSpeed)))))

(fn ConstructionScript)