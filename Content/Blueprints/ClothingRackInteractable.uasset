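; Interactable clothing rack that opens a hat selection menu when the player interacts with it.
; A sphere overlap shows a key-hint widget, refreshes its key and binds the character's interact event to the menu creation.
; Tick turns the hint toward the player's follow camera while in range.
; Leaving the sphere hides the hint and unbinds all interact events, and BeginPlay reuses that path to start hidden.
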(event OnComponentBeginOverlap(Sphere)
  (params (OverlappedComponent :type Primitive%20Component%20Object%20Reference) (OtherActor :type Actor%20Object%20Reference) (OtherComp :type Primitive%20Component%20Object%20Reference) (OtherBodyIndex :type Integer) (bFromSweep :type Boolean) (SweepResult :type Hit%20Result%20Structure%20%28by%20ref%29))
  (bind _widget (Variables|Default|GetWidget))
  ;[0.2462 0.6038 1] Widget Key Hint
  (bind _asbp_third_person_character (Utilities|Casting|CastToBP_ThirdPersonCharacter OtherActor))
  (if (Pawn|IsLocalPlayerController (Game|GetPlayerController 0))
    (bind _asbp_third_person_character_2 (Utilities|Casting|CastToBP_ThirdPersonCharacter (Game|GetPlayerCharacter 0)))
    (Development|SetHiddeninGame _widget false false)
    (Variables|Default|SetPlayer%20in%20Sphere true)
    (EventDispatchers|BindEventtoInteractEvent _asbp_third_person_character (delegate Custom|ToggleRadioEvent))
    (bind _aswdp_key_hint_1 (Utilities|Casting|CastToWDP_KeyHint1 (UserInterface|GetWidget _widget)))
    (Default|UpdateKey _aswdp_key_hint_1)))

(event OnComponentEndOverlap(Sphere)
  (params (OverlappedComponent :type Primitive%20Component%20Object%20Reference) (OtherActor :type Actor%20Object%20Reference) (OtherComp :type Primitive%20Component%20Object%20Reference) (OtherBodyIndex :type Integer))
  ;[0.2462 0.6038 1] Widget Key Hint
  (bind _asbp_third_person_character (Utilities|Casting|CastToBP_ThirdPersonCharacter OtherActor))
  (if (Pawn|IsLocalPlayerController (Game|GetPlayerController 0))
    (Development|SetHiddeninGame (Variables|Default|GetWidget) true false)
    (Variables|Default|SetPlayer%20in%20Sphere false)
    (if (Utilities|IsValid _asbp_third_person_character)
      (EventDispatchers|UnbindallEventsfromInteractEvent _asbp_third_person_character))))

(event Custom|ToggleRadioEvent
  (params (Host :type Boolean))
  ;[0.2462 0.6038 1] Widget Key Hint
  ;;[1 0.1176 0.9569] Interact with Device
  (bind _returnvalue (UserInterface|CreateWidget "/Game/UserInterface/HatSelection.HatSelection_C"))
  (UserInterface|Viewport|AddtoViewport _returnvalue 0))

(event EventTick
  (params (DeltaSeconds :type Float%20%28single-precision%29))
  (bind _widget (Variables|Default|GetWidget))
  ;[0.2462 0.6038 1] Widget Key Hint
  (if (and (Variables|Default|GetPlayer%20in%20Sphere) (Utilities|IsValid (stale OnComponentBeginOverlap(Sphere) _asbp_third_person_character)))
    (Transformation|SetWorldRotation _widget (Math|Rotator|FindLookatRotation (Transformation|GetWorldLocation _widget) (Transformation|GetWorldLocation (Variables|/Script/RoomOne.RoomOneCharacter|GetFollowCamera (stale OnComponentBeginOverlap(Sphere) _asbp_third_person_character_2)))) false false)))

(event EventBeginPlay
  ;[0.2462 0.6038 1] Widget Key Hint
  (Development|SetHiddeninGame (Variables|Default|GetWidget) true false)
  (Variables|Default|SetPlayer%20in%20Sphere false)
  (if (Utilities|IsValid (stale OnComponentEndOverlap(Sphere) _asbp_third_person_character))
    (EventDispatchers|UnbindallEventsfromInteractEvent (stale OnComponentEndOverlap(Sphere) _asbp_third_person_character))))

(fn ConstructionScript)