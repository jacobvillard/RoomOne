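; Server-side game manager for the King of the Boxes cube mode, running a timed match from waiting lobby to level restart.
; BeginPlay polls each tick until the expected player count or a timeout, then calls GameStart on each character.
; Tick calls EndGame when time expires, which picks the top Score, announces the winner and reloads the map via ServerTravel.
; Status messages reach players through each controller's AC_ChatPC multicast.
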(event Custom|EndGame
  (if (stale _output_get)
    (bind _output_get (Variables|Default|SetGameInProgress false))
    (bind _outactors (Actor|GetAllActorsOfClass "/Game/Blueprints/Characters/Goblin/BP_ThirdPersonCharacter_ChildKingOfTheBoxes.BP_ThirdPersonCharacter_ChildKingOfTheBoxes_C"))
    (for (_array_element _array_index) _outactors
      (if (== _array_index 0)
        (bind _output_get_2 (Variables|Default|SetHighscore _array_element))
        (elif (>= (Variables|/Game/Blueprints/Characters/Goblin/BP_ThirdPersonCharacter_ChildKingOfTheBoxes.BP_ThirdPersonCharacter_ChildKingOfTheBoxes_C|GetScore _array_element) (Variables|/Game/Blueprints/Characters/Goblin/BP_ThirdPersonCharacter_ChildKingOfTheBoxes.BP_ThirdPersonCharacter_ChildKingOfTheBoxes_C|GetScore _output_get_2))
          (bind _output_get_3 (Variables|Default|SetHighscore _array_element)))))
    (bind _outactors_2 (Actor|GetAllActorsOfClass "/Game/Blueprints/Systems/Chat/BP_GamePC.BP_GamePC_C")) ; Get all players
    (for _array_element_2 _outactors_2
      (Default|MulticastSystemMessage (Actor|GetComponentbyClass _array_element_2 "/Game/Blueprints/Systems/Chat/AC_ChatPC.AC_ChatPC_C") (Utilities|String|Append (Variables|/Game/Blueprints/Characters/Goblin/BP_ThirdPersonCharacter.BP_ThirdPersonCharacter_C|GetNameStr _output_get_3) " wins with " (Utilities|String|ToString(Integer) (Variables|/Game/Blueprints/Characters/Goblin/BP_ThirdPersonCharacter_ChildKingOfTheBoxes.BP_ThirdPersonCharacter_ChildKingOfTheBoxes_C|GetScore _output_get_3)) " points!") "(R=0.000000,G=1.000000,B=0.180450,A=1.000000)") ; Broadcast the message to all players
      ;[0.15 0.15 0.15 0.5] Show end screen, then restart level
      (Utilities|Time|ClearTimerbyFunctionName 0 "TimeLeft")
      (bind _asgame_instance_bp (Utilities|Casting|CastToGameInstanceBP (Game|GetGameInstance)))
      (bind _returnvalue (Class|GameModeBase|GetNumPlayers (Game|GetGameMode)))
      (Variables|/Game/Core/GameInstance/GameInstanceBP.GameInstanceBP_C|SetNumOfPlayers _asgame_instance_bp _returnvalue)
      (bind _outactors_3 (Actor|GetAllActorsOfClass "/Game/Blueprints/Systems/Chat/BP_GamePC.BP_GamePC_C")) ; Get all players
      (for _array_element_3 _outactors_3
        (Default|MulticastSystemMessage (Actor|GetComponentbyClass _array_element_3 "/Game/Blueprints/Systems/Chat/AC_ChatPC.AC_ChatPC_C") (Utilities|String|Append "Restart in " (Utilities|String|ToString(Integer) (Class|KismetMathLibrary|Round64 (Variables|Default|GetTimeUntilRestart))) " seconds")) ; Broadcast the message to all players
      )
      (Utilities|FlowControl|Delay (Variables|Default|GetTimeUntilRestart))
      (bind _returnvalue_2 (Game|GetCurrentLevelName true))
      (Development|ExecuteConsoleCommand (Utilities|String|Append "ServerTravel  /Game/ThirdPerson/Maps/" _returnvalue_2 "?listen") 0) ; Restart level
    )))

(event Custom|BroadcastStatus
  (bind _outactors (Actor|GetAllActorsOfClass "/Game/Blueprints/Systems/Chat/BP_GamePC.BP_GamePC_C")) ; Get all players
  (for _array_element _outactors
    (Default|MulticastSystemMessage (Actor|GetComponentbyClass _array_element "/Game/Blueprints/Systems/Chat/AC_ChatPC.AC_ChatPC_C") (Utilities|String|Append "Waiting for players " (Utilities|String|ToString(Integer) (stale EventBeginPlay _returnvalue)) "/" (Utilities|String|ToString(Integer) (Variables|/Game/Core/GameInstance/GameInstanceBP.GameInstanceBP_C|GetNumOfPlayers (stale EventBeginPlay _asgame_instance_bp))) ". Timeout in " (Utilities|String|ToString(Integer) (Class|KismetMathLibrary|Round64 (- (Variables|Default|GetGameTimeoutStart) (Actor|GetGameTimeSinceCreation))))) "(R=1.000000,G=0.000000,B=0.000000,A=1.000000)") ; Broadcast the message to all players
  ))

(event EventBeginPlay
  ;[0.15 0.15 0.15 0.5] Wait for all players or 60 seconds then select the seeker and start game
  (Utilities|IsSever
    (:Authority
      (Utilities|Time|SetTimerbyEvent (delegate Custom|BroadcastStatus) 5.0 true)
      (bind _asgame_instance_bp (Utilities|Casting|CastToGameInstanceBP (Game|GetGameInstance) :!label _label))
      (bind _returnvalue (Class|GameModeBase|GetNumPlayers (Game|GetGameMode)))
      (if (or (== _returnvalue (Variables|/Game/Core/GameInstance/GameInstanceBP.GameInstanceBP_C|GetNumOfPlayers _asgame_instance_bp)) (>= (Actor|GetGameTimeSinceCreation) (Variables|Default|GetGameTimeoutStart)))
        (Utilities|FlowControl|Delay 1.0)
        (Variables|Default|SetCurrentTimeStartTime (Actor|GetGameTimeSinceCreation))
        (Variables|Default|SetGameInProgress true)
        (Utilities|Time|ClearTimerbyFunctionName 0 "BroadcastStatus")
        (bind _outactors (Actor|GetAllActorsOfClass "/Game/Blueprints/Systems/Chat/BP_GamePC.BP_GamePC_C")) ; Get all players
        (for _array_element _outactors
          (Default|MulticastSystemMessage (Actor|GetComponentbyClass _array_element "/Game/Blueprints/Systems/Chat/AC_ChatPC.AC_ChatPC_C") "Get the cube!" "(R=0.000000,G=1.000000,B=0.307065,A=1.000000)") ; Broadcast the message to all players
        )
        (bind _outactors_2 (Actor|GetAllActorsOfClass "/Game/Blueprints/Characters/Goblin/BP_ThirdPersonCharacter_ChildKingOfTheBoxes.BP_ThirdPersonCharacter_ChildKingOfTheBoxes_C"))
        (for _array_element_2 _outactors_2
          (Variables|/Game/Blueprints/Characters/Goblin/BP_ThirdPersonCharacter_ChildKingOfTheBoxes.BP_ThirdPersonCharacter_ChildKingOfTheBoxes_C|SetMatchSeconds _array_element_2 (Math|Float|Truncate (Variables|Default|GetGameTime)))
          (Default|GameStart _array_element_2))
        (else
          (Utilities|FlowControl|DelayUntilNextTick)
          (goto _label))))))

(event EventTick
  (params (DeltaSeconds :type Float%20%28single-precision%29))
  (Utilities|IsSever
    (:Authority
      (if (Variables|Default|GetGameInProgress)
        (if (>= (- (Actor|GetGameTimeSinceCreation) (Variables|Default|GetCurrentTimeStartTime)) (Variables|Default|GetGameTime))
          (CallFunction|EndGame))))))

(fn ConstructionScript)

(fn RandomPlayer
  (return (Game|GetPlayerCharacter (.OutIndex (Utilities|Array|Random (Variables|/Script/Engine.GameStateBase|GetPlayerArray (Game|GetGameState)))))))