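; Server-side manager for an Infected tag mode that runs each round from lobby wait to level restart.
; It waits for the expected player count or a timeout, then picks a random player as Infected and freezes them for a head start.
; Authority-only Tick ends the round when all players are seekers or time expires.
; Chat components broadcast status and results, and EndGame saves the player count to the GameInstance before ServerTravel reloads the map.
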(event Custom|EndGame
  ;[0.15 0.15 0.15 0.5] Show end screen, then restart level
  (Variables|Default|SetGameInProgress false)
  (Utilities|Time|ClearTimerbyFunctionName 0 "TimeLeft")
  (bind _asgame_instance_bp (Utilities|Casting|CastToGameInstanceBP (Game|GetGameInstance)))
  (bind _returnvalue (Class|GameModeBase|GetNumPlayers (Game|GetGameMode)))
  (Variables|/Game/Core/GameInstance/GameInstanceBP.GameInstanceBP_C|SetNumOfPlayers _asgame_instance_bp _returnvalue)
  (bind _outactors (Actor|GetAllActorsOfClass "/Game/Blueprints/Systems/Chat/BP_GamePC.BP_GamePC_C")) ; Get all players
  (for _array_element _outactors
    (Default|MulticastSystemMessage (Actor|GetComponentbyClass _array_element "/Game/Blueprints/Systems/Chat/AC_ChatPC.AC_ChatPC_C") (Utilities|String|Append "Restart in " (Utilities|String|ToString(Integer) (Class|KismetMathLibrary|Round64 (Variables|Default|GetTimeUntilRestart))) " seconds")) ; Broadcast the message to all players
  )
  (Utilities|FlowControl|Delay (Variables|Default|GetTimeUntilRestart))
  (bind _returnvalue_2 (Game|GetCurrentLevelName true))
  (Development|ExecuteConsoleCommand (Utilities|String|Append "ServerTravel  /Game/ThirdPerson/Maps/" _returnvalue_2 "?listen") 0) ; Restart level
)

(event Custom|BroadcastStatus
  ;[0 1 0] Wait for all players or 60 seconds
  (bind _outactors (Actor|GetAllActorsOfClass "/Game/Blueprints/Systems/Chat/BP_GamePC.BP_GamePC_C")) ; Get all players
  (for _array_element _outactors
    (Default|MulticastSystemMessage (Actor|GetComponentbyClass _array_element "/Game/Blueprints/Systems/Chat/AC_ChatPC.AC_ChatPC_C") (Utilities|String|Append "Waiting for players " (Utilities|String|ToString(Integer) (stale EventBeginPlay _returnvalue)) "/" (Utilities|String|ToString(Integer) (Variables|/Game/Core/GameInstance/GameInstanceBP.GameInstanceBP_C|GetNumOfPlayers (stale EventBeginPlay _asgame_instance_bp))) ". Timeout in " (Utilities|String|ToString(Integer) (Class|KismetMathLibrary|Round64 (- (Variables|Default|GetGameTimeoutStart) (Actor|GetGameTimeSinceCreation))))) "(R=0.000000,G=0.000000,B=0.000000,A=1.000000)") ; Broadcast the message to all players
  ))

(event Custom|TimeLeft
  ;[0 1 0] HandleSeekr
  (bind _outactors (Actor|GetAllActorsOfClass "/Game/Blueprints/Systems/Chat/BP_GamePC.BP_GamePC_C")) ; Get all players
  (for _array_element _outactors
    (Default|MulticastSystemMessage (Actor|GetComponentbyClass _array_element "/Game/Blueprints/Systems/Chat/AC_ChatPC.AC_ChatPC_C") (Utilities|String|Append (Utilities|String|ToString(Integer) (Class|KismetMathLibrary|Round64 (- (Variables|Default|GetGameTime) (- (Actor|GetGameTimeSinceCreation) (Variables|Default|GetCurrentTimeStartTime))))) " seconds left!") "(R=0.274610,G=0.218750,B=1.000000,A=1.000000)") ; Broadcast the message to all players
  ))

(event EventBeginPlay
  ;[0 1 0] Wait for all players or 60 seconds
  (if (Ability|HasAuthority (Game|GetPlayerController 0))
    (Networking|SwitchHasAuthority
      (:Authority
        (Utilities|Time|SetTimerbyEvent (delegate Custom|BroadcastStatus) 5.0 true)
        (bind _asgame_instance_bp (Utilities|Casting|CastToGameInstanceBP (Game|GetGameInstance) :!label _label))
        (bind _returnvalue (Class|GameModeBase|GetNumPlayers (Game|GetGameMode)))
        (if (or (== _returnvalue (Variables|/Game/Core/GameInstance/GameInstanceBP.GameInstanceBP_C|GetNumOfPlayers _asgame_instance_bp)) (>= (Actor|GetGameTimeSinceCreation) (Variables|Default|GetGameTimeoutStart)))
          (Utilities|FlowControl|Delay 1.0)
          ;[0 1 0] HandleSeekr
          (bind _asbp_third_person_character_child_infected (Utilities|Casting|CastTo (CallFunction|RandomPlayer)))
          (CallFunction|ServerIAmSeeker _asbp_third_person_character_child_infected)
          (bind _outactors (Actor|GetAllActorsOfClass "/Game/Blueprints/Systems/Chat/BP_GamePC.BP_GamePC_C")) ; Get all players
          (for _array_element _outactors
            (Default|MulticastSystemMessage (Actor|GetComponentbyClass _array_element "/Game/Blueprints/Systems/Chat/AC_ChatPC.AC_ChatPC_C") (Utilities|String|Append (PlayerState|GetPlayerName (Variables|/Script/Engine.Pawn|GetPlayerState _asbp_third_person_character_child_infected)) " is infected! " "They will be released in " (Utilities|String|ToString(Float) (Variables|Default|GetHunterFrozenTime)) " seconds") "(R=0.000000,G=0.302327,B=1.000000,A=1.000000)") ; Broadcast the message to all players
          )
          (Utilities|Time|ClearTimerbyFunctionName 0 "BroadcastStatus")
          (Pawn|Components|CharacterMovement|SetMovementMode (Variables|/Script/Engine.Character|GetCharacterMovement _asbp_third_person_character_child_infected) "MOVE_None" 0)
          (bind _outactors_2 (Actor|GetAllActorsOfClass 0))
          (for _array_element_2 _outactors_2
            (Variables|Default|SetTimer _array_element_2 (Math|Float|Truncate (+ (Variables|Default|GetHunterFrozenTime) (Variables|Default|GetGameTime))))
            (if (!= _asbp_third_person_character_child_infected _array_element_2)
              (Variables|Default|SetRoleStr _array_element_2 "Survivor")
              (else
                (Variables|Default|SetRoleStr _array_element_2 "Infected"))))
          (Utilities|FlowControl|Delay (Variables|Default|GetHunterFrozenTime))
          (Pawn|Components|CharacterMovement|SetMovementMode (Variables|/Script/Engine.Character|GetCharacterMovement _asbp_third_person_character_child_infected) "MOVE_Falling" 0)
          (bind _outactors_3 (Actor|GetAllActorsOfClass "/Game/Blueprints/Systems/Chat/BP_GamePC.BP_GamePC_C")) ; Get all players
          (for _array_element_3 _outactors_3
            (Default|MulticastSystemMessage (Actor|GetComponentbyClass _array_element_3 "/Game/Blueprints/Systems/Chat/AC_ChatPC.AC_ChatPC_C") "Infected released good luck!" "(R=1.000000,G=0.000000,B=0.412543,A=1.000000)") ; Broadcast the message to all players
          )
          (Variables|Default|SetCurrentTimeStartTime (Actor|GetGameTimeSinceCreation))
          (Utilities|Time|SetTimerbyEvent (delegate Custom|TimeLeft) 3e+01 true)
          (Variables|Default|SetGameInProgress true)
          (CallFunction|ServerIAmSeeker _asbp_third_person_character_child_infected)
          (else
            (Utilities|FlowControl|DelayUntilNextTick)
            (goto _label)))))))

(event EventTick
  (params (DeltaSeconds :type Float%20%28single-precision%29))
  ;[0 1 0] Check if game is over
  (if (Variables|Default|GetGameInProgress)
    (Networking|SwitchHasAuthority
      (:Authority
        (Variables|Default|SetCounter 0)
        (bind _array_index (Utilities|Array|ForEachLoopwithBreak (Variables|/Script/Engine.GameStateBase|GetPlayerArray (Game|GetGameState)))
          (:LoopBody
            (bind _asbp_third_person_character_child_infected (Utilities|Casting|CastTo (Game|GetPlayerCharacter _array_index)))
            (if (Variables|Default|GetSeeker _asbp_third_person_character_child_infected)
              (Variables|Default|SetCounter (+ (Variables|Default|GetCounter) 1))))
          (:Completed
            (bind _returnvalue (Class|GameModeBase|GetNumPlayers (Game|GetGameMode)))
            (if (== _returnvalue (Variables|Default|GetCounter))
              (CallFunction|EndGame)
              (bind _outactors (Actor|GetAllActorsOfClass "/Game/Blueprints/Systems/Chat/BP_GamePC.BP_GamePC_C")) ; Get all players
              (for _array_element _outactors
                (Default|MulticastSystemMessage (Actor|GetComponentbyClass _array_element "/Game/Blueprints/Systems/Chat/AC_ChatPC.AC_ChatPC_C") "The Infected Win!" "(R=1.000000,G=0.000000,B=0.412543,A=1.000000)") ; Broadcast the message to all players
              )
              (elif (>= (- (Actor|GetGameTimeSinceCreation) (Variables|Default|GetCurrentTimeStartTime)) (Variables|Default|GetGameTime))
                (CallFunction|EndGame)
                (bind _outactors_2 (Actor|GetAllActorsOfClass "/Game/Blueprints/Systems/Chat/BP_GamePC.BP_GamePC_C")) ; Get all players
                (for _array_element_2 _outactors_2
                  (Default|MulticastSystemMessage (Actor|GetComponentbyClass _array_element_2 "/Game/Blueprints/Systems/Chat/AC_ChatPC.AC_ChatPC_C") "The Survivors Win!" "(R=0.000000,G=1.000000,B=0.056128,A=1.000000)") ; Broadcast the message to all players
                )))))))))

(fn ConstructionScript)

(fn RandomPlayer
  (return (Game|GetPlayerCharacter (.OutIndex (Utilities|Array|Random (Variables|/Script/Engine.GameStateBase|GetPlayerArray (Game|GetGameState)))))))