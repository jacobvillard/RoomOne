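; ChainsLinked is a rope-style actor that procedurally builds a hanging or loose physics chain from twenty chain link meshes.
; The construction script spawns physics-simulated static mesh links along X, rolling each a quarter turn from the last so they interlock visually.
; Each link gets a physics constraint joining it to the previous link, with collision between the pair disabled.
; The event graph holds no runtime logic.
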(event EventBeginPlay)

(event Collision|EventActorBeginOverlap
  (params (OtherActor :type Actor%20Object%20Reference)))

(event EventTick
  (params (DeltaSeconds :type Float%20%28single-precision%29)))

(fn ConstructionScript
  (for _index (range 1 20)
    (bind _returnvalue (AddComponent|AddStaticMeshComponent false (Math|Transform|MakeTransform (Math|Vector|MakeVector (Math|Conversions|ToFloat(Integer) (* _index 7)) 0.0 0.0) (Math|Rotator|MakeRotator (Math|Conversions|ToFloat(Integer) (* _index 90)) 0.0 0.0))))
    (bind _output_get (Variables|Default|SetStaticMesh _returnvalue))
    (bind _returnvalue_2 (Utilities|Array|Add (Variables|Default|GetMeshes) _output_get))
    (Variables|Default|SetCurrentIndex _returnvalue_2)
    (Components|StaticMesh|SetStaticMesh _output_get "/Game/Blueprints/Rope/ChainLink.ChainLink")
    (Physics|SetSimulatePhysics _output_get true)
    (Collision|SetCollisionEnabled _output_get "QueryAndPhysics")
    (bind _returnvalue_3 (AddComponent|AddPhysicsConstraintComponent false (Math|Transform|MakeTransform (- (.location (Transformation|GetRelativeTransform _output_get)) "100.000000,-0.000000,50.000000") "0, 0, 0" "1.000000,1.000000,1.000000")))
    (bind _output_get_2 (Variables|Default|SetPhysicsConstraint _returnvalue_3))
    (Utilities|Array|Add (Variables|Default|GetConstraints) _output_get_2)
    (if (and (Utilities|IsValid (Utilities|Array|Get(acopy) (Variables|Default|GetMeshes) (Variables|Default|GetCurrentIndex))) (Utilities|IsValid (Utilities|Array|Get(acopy) (Variables|Default|GetMeshes) (- (Variables|Default|GetCurrentIndex) 1))))
      (Class|PhysicsConstraintComponent|SetConstrainedComponents (Variables|Default|GetPhysicsConstraint) (Utilities|Array|Get(acopy) (Variables|Default|GetMeshes) (Variables|Default|GetCurrentIndex)) "None" (Utilities|Array|Get(acopy) (Variables|Default|GetMeshes) (- (Variables|Default|GetCurrentIndex) 1)) "None")
      (Class|PhysicsConstraintComponent|SetDisableCollision (Variables|Default|GetPhysicsConstraint) true))))