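; FixedRope is a rope actor that tethers two physics third-person characters and pulls one when the rope overstretches.
; After a startup delay it finds both players and pins its end spheres to their attach points.
; Each tick it sums distances along sampled bone components; beyond a maximum, it launches the slower player toward the bone near the other end.
; Only P2 also switches to custom movement mode when launched.
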(event Collision|EventActorBeginOverlap
  (params (OtherActor :type Actor%20Object%20Reference)))

(event EventTick
  (params (DeltaSeconds :type Float%20%28single-precision%29))
  (bind _p1 (Variables|Default|GetP1))
  (bind _bone_010 (Variables|Default|GetBone_010))
  (bind _p2 (Variables|Default|GetP2))
  (bind _bone_015 (Variables|Default|GetBone_015))
  (bind _bone_020 (Variables|Default|GetBone_020))
  (bind _bone_025 (Variables|Default|GetBone_025))
  (bind _bone_005 (Variables|Default|GetBone_005))
  (bind _returnvalue (Transformation|GetWorldLocation _bone_010))
  (bind _returnvalue_2 (Transformation|GetWorldLocation _bone_015))
  (bind _returnvalue_3 (Transformation|GetWorldLocation _bone_020))
  (bind _returnvalue_4 (Transformation|GetWorldLocation _bone_025))
  (bind _returnvalue_5 (Transformation|GetWorldLocation _bone_005))
  (if (Variables|Default|GetPlayersSet)
    (Transformation|SetWorldLocation (Variables|Default|GetStartSphere) (Transformation|GetWorldLocation (Variables|/Game/ThirdPerson/Blueprints/BP_ThirdPersonCharacterPhysics.BP_ThirdPersonCharacterPhysics_C|GetAttach (Variables|Default|GetP1))) false false)
    (Transformation|SetWorldLocation (Variables|Default|GetEndSphere) (Transformation|GetWorldLocation (Variables|/Game/ThirdPerson/Blueprints/BP_ThirdPersonCharacterPhysics.BP_ThirdPersonCharacterPhysics_C|GetAttach (Variables|Default|GetP2))) false false)
    (if (> (+ (Math|Vector|Distance(Vector) (Transformation|GetWorldLocation (Variables|Default|GetStartSphere)) _returnvalue_5) (Math|Vector|Distance(Vector) _returnvalue_5 _returnvalue) (Math|Vector|Distance(Vector) _returnvalue _returnvalue_2) (Math|Vector|Distance(Vector) _returnvalue_2 _returnvalue_3) (Math|Vector|Distance(Vector) _returnvalue_3 _returnvalue_4) (Math|Vector|Distance(Vector) _returnvalue_4 (Transformation|GetWorldLocation (Variables|Default|GetEndSphere)))) (Variables|Default|GetDistanceMax))
      (if (> (Math|Vector|VectorLength (Class|NavMovementComponent|GetVelocityforNavMovement (Variables|/Script/Engine.Character|GetCharacterMovement (Variables|Default|GetP2)))) (Math|Vector|VectorLength (Class|NavMovementComponent|GetVelocityforNavMovement (Variables|/Script/Engine.Character|GetCharacterMovement (Variables|Default|GetP1)))))
        (Character|LaunchCharacter _p1 (* (Math|Vector|GetUnitDirection(Vector) (Transformation|GetWorldLocation (Variables|/Game/ThirdPerson/Blueprints/BP_ThirdPersonCharacterPhysics.BP_ThirdPersonCharacterPhysics_C|GetAttach _p1)) (Transformation|GetWorldLocation (Variables|Default|GetBone_025))) (Variables|Default|GetLaunchMultiplier)) false false)
        (else
          (Character|LaunchCharacter _p2 (* (Math|Vector|GetUnitDirection(Vector) (Transformation|GetWorldLocation (Variables|/Game/ThirdPerson/Blueprints/BP_ThirdPersonCharacterPhysics.BP_ThirdPersonCharacterPhysics_C|GetAttach _p2)) (Transformation|GetWorldLocation (Variables|Default|GetBone_005))) (Variables|Default|GetLaunchMultiplier)) false false)
          (Pawn|Components|CharacterMovement|SetMovementMode (Variables|/Script/Engine.Character|GetCharacterMovement _p2) "MOVE_Custom" 0))))))

(event EventBeginPlay
  (Utilities|FlowControl|Delay 3.0)
  (bind _outactors (Actor|GetAllActorsOfClass "/Game/ThirdPerson/Blueprints/BP_ThirdPersonCharacterPhysics.BP_ThirdPersonCharacterPhysics_C"))
  (bind _output_get (Variables|Default|SetOut%20Actors _outactors))
  (bind _output_get_2 (Variables|Default|SetP1 (Utilities|Array|Get(acopy) _output_get)))
  (bind _output_get_3 (Variables|Default|SetP2 (Utilities|Array|Get(acopy) _output_get 1)))
  (Transformation|AttachComponentToComponent (Variables|Default|GetStartSphere) (Variables|/Game/ThirdPerson/Blueprints/BP_ThirdPersonCharacterPhysics.BP_ThirdPersonCharacterPhysics_C|GetAttach _output_get_2) "None" "SnapToTarget" "SnapToTarget" "KeepRelative" true)
  (Transformation|AttachComponentToComponent (Variables|Default|GetEndSphere) (Variables|/Game/ThirdPerson/Blueprints/BP_ThirdPersonCharacterPhysics.BP_ThirdPersonCharacterPhysics_C|GetAttach _output_get_3) "None" "SnapToTarget" "SnapToTarget" "KeepRelative" true)
  (Variables|Default|SetPlayersSet true))

(fn ConstructionScript)