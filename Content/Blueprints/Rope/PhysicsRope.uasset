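; Physics rope actor that tethers two BP_CustomCharacter players using a skeletal mesh and physics constraints.
; On BeginPlay it positions the Start and End constraints near the end bones, waits briefly, then takes the first two characters found.
; It moves itself to align the first bone with P1, then constrains each end bone to a player's capsule.
; Tick does nothing; the rope-length check that pulls players with force is disconnected.
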(event Custom|SetStartLoc
  (Transformation|SetActorLocation (+ (Transformation|GetActorLocation) (- (Transformation|GetWorldLocation (Variables|/Script/Engine.Character|GetCapsuleComponent (Variables|Default|GetP1))) (Transformation|GetSocketLocation (Variables|Default|GetSkeletalMesh) "Bone"))) false true))

(event EventBeginPlay
  (bind _skeletalmesh (Variables|Default|GetSkeletalMesh))
  (bind _skeletalmesh_2 (Variables|Default|GetSkeletalMesh))
  (Transformation|SetWorldLocation (Variables|Default|GetStart) (- (Transformation|GetSocketLocation _skeletalmesh_2 "Bone") "0.000000,0.000000,50.000000") false true)
  (Transformation|SetWorldLocation (Variables|Default|GetEnd) (+ (Transformation|GetSocketLocation _skeletalmesh_2 "Bone_030") "0.000000,0.000000,50.000000") false true)
  (Utilities|FlowControl|Delay 3.0)
  (Variables|Default|SetPlayersSet true)
  (bind _outactors (Actor|GetAllActorsOfClass "/Game/ThirdPerson/Blueprints/BP_CustomCharacter.BP_CustomCharacter_C"))
  (bind _output_get (Variables|Default|SetOut%20Actors _outactors))
  (bind _output_get_2 (Variables|Default|SetP1 (Utilities|Array|Get(acopy) _output_get)))
  (bind _output_get_3 (Variables|Default|SetP2 (Utilities|Array|Get(acopy) _output_get 1)))
  (CallFunction|SetStartLoc)
  (Class|PhysicsConstraintComponent|SetConstrainedComponents (Variables|Default|GetStart) (Variables|/Script/Engine.Character|GetCapsuleComponent _output_get_2) "None" _skeletalmesh "Bone")
  (Class|PhysicsConstraintComponent|SetConstrainedComponents (Variables|Default|GetEnd) (Variables|/Script/Engine.Character|GetCapsuleComponent _output_get_3) "None" _skeletalmesh "Bone_030"))

(event Collision|EventActorBeginOverlap
  (params (OtherActor :type Actor%20Object%20Reference)))

(event EventTick
  (params (DeltaSeconds :type Float%20%28single-precision%29))
  (if (Variables|Default|GetPlayersSet)
    _))

(fn ConstructionScript)