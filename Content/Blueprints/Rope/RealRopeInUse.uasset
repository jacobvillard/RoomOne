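; Rope actor that tethers two players at the hips and lets each interact to pull the other.
; A looping timer rebuilds a three-point spline with distance-based sag, lays instanced rope meshes along it, and turns pull widgets toward the opposite player's camera.
; Beyond MaxLength, the server launches falling players toward each other and stops grounded ones, adding a half-force pull if further overstretched.
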(event Custom|InteractedPlayer1
  (params (Host :type Boolean))
  (CallFunction|PullPlayer2))

(event Custom|UpdateRope
  (bind _player1 (Variables|Default|GetPlayer1))
  (bind _player2 (Variables|Default|GetPlayer2))
  (bind _charactermovement (Variables|/Script/Engine.Character|GetCharacterMovement _player2))
  (bind _charactermovement_2 (Variables|/Script/Engine.Character|GetCharacterMovement _player1))
  (if (CallFunction|ArePlayersValid)
    (Utilities|FlowControl|Sequence
      (:then_0
        (Utilities|FlowControl|DoOnce false
          (:Completed
            (EventDispatchers|BindEventtoInteractEvent (Variables|Default|GetPlayer1) (delegate Custom|InteractedPlayer1))
            (EventDispatchers|BindEventtoInteractEvent (Variables|Default|GetPlayer2) (delegate Custom|InteractedPlayer2)))))
      (:then_1
        (CallFunction|SetSplinePoints)
        (CallFunction|AddSplineMesh)
        (CallFunction|RotateWidgets)
        (Networking|SwitchHasAuthority
          (:Authority
            (Default|ServerRopeWidgets (Variables|Default|GetPlayer1) (Variables|Default|GetPlayer2))
            (Default|ServerRopeWidgets (Variables|Default|GetPlayer2) (Variables|Default|GetPlayer1))
            (if (> (.Distance (CallFunction|GetPlayerLocationsandDistance)) (Variables|Default|GetMaxLength))
              (Utilities|FlowControl|Sequence
                (:then_0
                  (if (AI|Components|NavMovement|IsFalling _charactermovement_2)
                    (Character|LaunchCharacter (Variables|Default|GetPlayer1) (* (.Direction (CallFunction|GetPlayerLocationsandDistance)) (Variables|Default|GetPullForce)) true true)
                    (else
                      (Components|Movement|StopMovementImmediately _charactermovement_2)
                      (if (> (.Distance (CallFunction|GetPlayerLocationsandDistance)) (+ (Variables|Default|GetMaxLength) 1e+02))
                        (Character|LaunchCharacter (Variables|Default|GetPlayer1) (/ (* (.Direction (CallFunction|GetPlayerLocationsandDistance)) (Variables|Default|GetPullForce)) 2.0) true true)))))
                (:then_1
                  (if (AI|Components|NavMovement|IsFalling _charactermovement)
                    (Character|LaunchCharacter _player2 (* (* (.Direction (CallFunction|GetPlayerLocationsandDistance)) -1.0) (Variables|Default|GetPullForce)) true true)
                    (else
                      (Components|Movement|StopMovementImmediately _charactermovement)
                      (if (> (.Distance (CallFunction|GetPlayerLocationsandDistance)) (+ (Variables|Default|GetMaxLength) 1e+02))
                        (Character|LaunchCharacter (Variables|Default|GetPlayer2) (/ (* (* (.Direction (CallFunction|GetPlayerLocationsandDistance)) -1.0) (Variables|Default|GetPullForce)) 2.0) true true)))))))))))))

(event Custom|InteractedPlayer2
  (params (Host :type Boolean))
  (CallFunction|PullPlayer1))

(event Custom|PullPlayer1
  (if (Variables|/Game/ThirdPerson/Blueprints/BP_ThirdPersonCharacter.BP_ThirdPersonCharacter_C|GetCanPullOtherPlayer (Variables|Default|GetPlayer2))
    (Character|LaunchCharacter (Variables|Default|GetPlayer1) (* (.Direction (CallFunction|GetPlayerLocationsandDistance)) (Variables|Default|GetPullForce)) true true)
    (Development|PrintString "PullPlayer1")))

(event Custom|PullPlayer2
  (if (Variables|/Game/ThirdPerson/Blueprints/BP_ThirdPersonCharacter.BP_ThirdPersonCharacter_C|GetCanPullOtherPlayer (Variables|Default|GetPlayer1))
    (Character|LaunchCharacter (Variables|Default|GetPlayer2) (* (* (.Direction (CallFunction|GetPlayerLocationsandDistance)) -1.0) (Variables|Default|GetPullForce)) true true)
    (Development|PrintString "PullPlayer2")))

(event EventBeginPlay
  (Utilities|Time|SetTimerbyFunctionName 0 "UpdateRope" 0.025 true true))

(fn ConstructionScript
  (bind _ropemesh (Variables|Default|GetRopeMesh))
  (bind _returnvalue (StaticMesh|GetBoundingBox _ropemesh))
  (bind (_min _max) (Utilities|Struct|BreakBox _returnvalue))
  (Components|StaticMesh|SetStaticMesh (Variables|Default|GetInstancedStaticMesh) (Variables|Default|GetRopeMesh))
  (Variables|Default|SetSpacing (+ (.Z (Math|Vector|BreakVector (- _max _min))) (Variables|Default|GetOffset))))

(fn OnRepPlayer2)

(fn OnRepPlayer1)

(fn AddSplineMesh
  (bind _spacing (Variables|Default|GetSpacing))
  (Components|InstancedStaticMesh|ClearInstances (Variables|Default|GetInstancedStaticMesh))
  (bind _output_get (LocalVariables|SetNumInstances (Math|Float|Floor (/ (Spline|GetSplineLength (Variables|Default|GetSpline)) (Variables|Default|GetSpacing)))))
  (for _index (range 0 _output_get)
    (Components|InstancedStaticMesh|AddInstance (Variables|Default|GetInstancedStaticMesh) (Math|Transform|MakeTransform (CallFunction|GetLocationatIndexLocal _index _spacing) (Math|Rotator|MakeRotfromZ (- (CallFunction|GetLocationatIndexLocal (+ _index 1) _spacing) (CallFunction|GetLocationatIndexLocal _index _spacing)))) false)))

(fn SetSplinePoints
  (bind (_sag _distance _p1location _p2location) (CallFunction|GetPlayerLocationsandDistance))
  (Spline|ClearSplinePoints (Variables|Default|GetSpline) false)
  (Spline|AddSplinePoint (Variables|Default|GetSpline) (.P2Location (CallFunction|GetPlayerLocationsandDistance)) "World" false)
  (Spline|AddSplinePoint (Variables|Default|GetSpline) (CallFunction|GetMiddlePoint _p1location _p2location _sag) "World" false)
  (Spline|AddSplinePoint (Variables|Default|GetSpline) (.P1Location (CallFunction|GetPlayerLocationsandDistance)) "World" false)
  (for _index (range 0 (- (Spline|GetNumberOfSplinePoints (Variables|Default|GetSpline)) 1))
    (Spline|SetSplinePointType (Variables|Default|GetSpline) _index "Curve" true)))

(fn GetLocationatIndexLocal
  (params (A :type Integer) (Spacing :type Float%20%28double-precision%29))
  (return (Spline|GetLocationatDistanceAlongSpline (Variables|Default|GetSpline) (* A Spacing) "Local")))

(fn ArePlayersValid
  (return (and (Utilities|IsValid (Variables|Default|GetPlayer1)) (Utilities|IsValid (Variables|Default|GetPlayer2)))))

(fn GetPlayerLocationsandDistance
  (bind _player1 (Variables|Default|GetPlayer1))
  (bind _player2 (Variables|Default|GetPlayer2))
  (bind _mesh (Variables|/Script/Engine.Character|GetMesh _player2))
  (bind _mesh_2 (Variables|/Script/Engine.Character|GetMesh _player1))
  (bind _returnvalue (Transformation|GetSocketLocation _mesh_2 "Hips"))
  (bind _returnvalue_2 (Transformation|GetSocketLocation _mesh "Hips"))
  (bind _returnvalue_3 (Math|Vector|Distance(Vector) _returnvalue _returnvalue_2))
  (return (Math|Float|Clamp(Float) (* (/ (Variables|Default|GetMaxLength) _returnvalue_3) (Variables|Default|GetSagMultiplier)) 0.0 (Variables|Default|GetMaxSag)) _returnvalue_3 _returnvalue _returnvalue_2 (Math|Vector|GetUnitDirection(Vector) _returnvalue _returnvalue_2)))

(fn GetMiddlePoint
  (params (A :type Vector) (B :type Vector) (Sag :type Float%20%28double-precision%29))
  (return (- (/ (+ A B) 2.0) (Math|Vector|MakeVector 0.0 0.0 Sag))))

(fn GetLocationatIndexWorld
  (params (A :type Integer) (Spacing :type Float%20%28double-precision%29))
  (return (Spline|GetLocationatDistanceAlongSpline (Variables|Default|GetSpline) (* A Spacing) "World")))

(fn RotateWidgets
  (bind _player2 (Variables|Default|GetPlayer2))
  (bind _player1 (Variables|Default|GetPlayer1))
  (bind _ropepullwidget (Variables|/Game/ThirdPerson/Blueprints/BP_ThirdPersonCharacter.BP_ThirdPersonCharacter_C|GetRopePullWidget _player2))
  (bind _ropepullwidget_2 (Variables|/Game/ThirdPerson/Blueprints/BP_ThirdPersonCharacter.BP_ThirdPersonCharacter_C|GetRopePullWidget _player1))
  (Transformation|SetWorldRotation _ropepullwidget_2 (Math|Rotator|FindLookatRotation (Transformation|GetWorldLocation _ropepullwidget_2) (Transformation|GetWorldLocation (Variables|/Script/RoomOne.RoomOneCharacter|GetFollowCamera (Variables|Default|GetPlayer2)))) false false)
  (Transformation|SetWorldRotation _ropepullwidget (Math|Rotator|FindLookatRotation (Transformation|GetWorldLocation _ropepullwidget) (Transformation|GetWorldLocation (Variables|/Script/RoomOne.RoomOneCharacter|GetFollowCamera (Variables|Default|GetPlayer1)))) false false))