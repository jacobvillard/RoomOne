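; Trigger actor that ropes player characters together when a BP_ThirdPersonCharacter overlaps its sphere.
; On overlap it destroys existing ropes, then the authority shows a CircleOrLine widget to choose layout, sag, length and pull force.
; The choice gathers all characters and spawns RealRopeInUse actors between consecutive players, passing them those settings and the rope mesh.
; Circle layout wraps the last player to the first; line layout leaves the ends open.
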(event OnComponentBeginOverlap(Sphere)
  (params (OverlappedComponent :type Primitive%20Component%20Object%20Reference) (OtherActor :type Actor%20Object%20Reference) (OtherComp :type Primitive%20Component%20Object%20Reference) (OtherBodyIndex :type Integer) (bFromSweep :type Boolean) (SweepResult :type Hit%20Result%20Structure%20%28by%20ref%29))
  (bind _returnvalue (Game|GetPlayerController 0))
  (bind _ropes (Variables|Initialization|GetRopes))
  (Utilities|Casting|CastToBP_ThirdPersonCharacter OtherActor)
  (for _array_element _ropes
    (Actor|DestroyActor _array_element))
  (Utilities|Array|Clear _ropes)
  (Utilities|Array|Clear (Variables|Initialization|GetPlayers))
  (Networking|SwitchHasAuthority
    (:Authority
      (bind _returnvalue_2 (UserInterface|CreateWidget "/Game/UserInterface/CircleOrLine.CircleOrLine_C"))
      (UserInterface|Viewport|AddtoPlayerScreen _returnvalue_2)
      (Input|SetInputModeUIOnly _returnvalue _returnvalue_2 "DoNotLock" true)
      (Variables|/Script/Engine.PlayerController|SetbShowMouseCursor _returnvalue true)
      (EventDispatchers|BindEventtoLineType _returnvalue_2 (delegate Custom|ChangeType)))))

(event Custom|ChangeType
  (params (CircleOrLine :type Integer) (Sag :type Float%20%28double-precision%29) (Length :type Float%20%28double-precision%29) (Force :type Float%20%28double-precision%29))
  (bind _returnvalue (Game|GetPlayerController 0))
  (Variables|Customisation|SetMaxSag Sag)
  (Variables|Customisation|SetRopeLength Length)
  (Variables|Customisation|SetPullForce Force)
  (Variables|Customisation|SetCircle1Line2 CircleOrLine)
  (Widget|RemovefromParent (stale OnComponentBeginOverlap(Sphere) _returnvalue_2))
  (Input|SetInputModeGameOnly _returnvalue true)
  (Variables|/Script/Engine.PlayerController|SetbShowMouseCursor _returnvalue false)
  (Utilities|FlowControl|Sequence
    (:then_0
      (Networking|SwitchHasAuthority
        (:Authority
          (bind _outactors (Actor|GetAllActorsOfClass "/Game/ThirdPerson/Blueprints/BP_ThirdPersonCharacter.BP_ThirdPersonCharacter_C"))
          (Variables|Initialization|SetPlayers _outactors))))
    (:then_1
      (for _index (range 0 (- (Utilities|Array|Length (Variables|Initialization|GetPlayers)) (Variables|Customisation|GetCircle1Line2)))
        (Variables|Initialization|SetIndex _index)
        (bind _returnvalue_2 (Game|SpawnActorfromClass "/Game/Blueprints/Rope/RealRopeInUse.RealRopeInUse_C" (Transformation|GetActorTransform) "AlwaysSpawn" "MultiplyWithRoot" 0 0))
        (Variables|Initialization|SetCurrentRope _returnvalue_2)
        (CallFunction|SetRopeFloats)
        (Variables|/Game/Blueprints/Rope/RealRopeInUse.RealRopeInUse_C|SetRopeMesh (Variables|Initialization|GetCurrentRope) "/Game/Blueprints/Rope/RopeSM.RopeSM")
        (CallFunction|SetRopePlayers)
        (Utilities|Array|Add (Variables|Initialization|GetRopes) (Variables|Initialization|GetCurrentRope))))))

(event EventBeginPlay)

(event Collision|EventActorBeginOverlap
  (params (OtherActor :type Actor%20Object%20Reference)))

(event EventTick
  (params (DeltaSeconds :type Float%20%28single-precision%29)))

(fn ConstructionScript)

(fn SetRopeFloats
  (Variables|/Game/Blueprints/Rope/RealRopeInUse.RealRopeInUse_C|SetMaxLength (Variables|Initialization|GetCurrentRope) (Variables|Customisation|GetRopeLength))
  (Variables|/Game/Blueprints/Rope/RealRopeInUse.RealRopeInUse_C|SetMaxSag (Variables|Initialization|GetCurrentRope) (Variables|Customisation|GetMaxSag))
  (Variables|/Game/Blueprints/Rope/RealRopeInUse.RealRopeInUse_C|SetPullForce (Variables|Initialization|GetCurrentRope) (Variables|Customisation|GetPullForce)))

(fn SetRopePlayers
  (bind _index (Variables|Initialization|GetIndex))
  (bind _returnvalue (+ _index 1))
  (Utilities|IsValid (Utilities|Array|Get(acopy) (Variables|Initialization|GetPlayers) _returnvalue)
    (:Is%20Valid
      (Variables|Initialization|SetPlayer2Index _returnvalue))
    (:Is%20Not%20Valid
      (Variables|Initialization|SetPlayer2Index 0)))
  (bind _output_get (Variables|/Game/Blueprints/Rope/RealRopeInUse.RealRopeInUse_C|SetPlayer1 (Variables|Initialization|GetCurrentRope) (Utilities|Array|Get(acopy) (Variables|Initialization|GetPlayers) (Variables|Initialization|GetIndex))))
  (bind _output_get_2 (Variables|/Game/Blueprints/Rope/RealRopeInUse.RealRopeInUse_C|SetPlayer2 (Variables|Initialization|GetCurrentRope) (Utilities|Array|Get(acopy) (Variables|Initialization|GetPlayers) (Variables|Initialization|GetPlayer2Index))))
  (return _output_get _output_get_2))