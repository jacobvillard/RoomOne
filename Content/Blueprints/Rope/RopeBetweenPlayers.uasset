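; Rope actor that visually tethers two players and pulls them together when stretched past a maximum length.
; A looping timer rebuilds a three-point spline between their hip sockets, sagging more as they get closer.
; Instanced static meshes are respaced along that spline on each update.
; When the spline exceeds the limit, the authority pulls both players inward, using forces on physics-simulated meshes or character launches otherwise.
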(event Custom|UpdateRope
  (bind (_sag _distance _p1location _p2location) (CallFunction|GetPlayerLocationsandDistance))
  (bind _player1 (Variables|Default|GetPlayer1))
  (bind _player2 (Variables|Default|GetPlayer2))
  (bind _player1_2 (Variables|Default|GetPlayer1))
  (bind _pullforce (Variables|Default|GetPullForce))
  (bind _player2_2 (Variables|Default|GetPlayer2))
  (bind _returnvalue (Math|Vector|GetUnitDirection(Vector) _p1location _p2location))
  (bind _mesh (Variables|/Script/Engine.Character|GetMesh _player2))
  (bind _mesh_2 (Variables|/Script/Engine.Character|GetMesh _player1_2))
  (bind _returnvalue_2 (* _returnvalue _pullforce))
  (bind _returnvalue_3 (* _returnvalue_2 -1.0))
  (if (CallFunction|ArePlayersValid)
    (CallFunction|SetSplinePoints)
    (CallFunction|AddSplineMesh)
    (Networking|SwitchHasAuthority
      (:Authority
        (if (> (Spline|GetSplineLength (Variables|Default|GetSpline)) (Variables|Default|GetMaxLength))
          (Utilities|FlowControl|Sequence
            (:then_0
              (if (Physics|IsSimulatingPhysics _mesh_2 "None")
                (Physics|AddForce _mesh_2 (* _returnvalue_2 3e+02) "None" true)
                (else
                  (Character|LaunchCharacter _player1 _returnvalue_2 true true)
                  (Pawn|Components|CharacterMovement|SetMovementMode (Variables|/Script/Engine.Character|GetCharacterMovement _player1) "MOVE_Walking" 0))))
            (:then_1
              (if (Physics|IsSimulatingPhysics _mesh "None")
                (Physics|AddForce _mesh (* _returnvalue_3 3e+02) "None" true)
                (else
                  (Character|LaunchCharacter _player2_2 _returnvalue_3 true true)
                  (Pawn|Components|CharacterMovement|SetMovementMode (Variables|/Script/Engine.Character|GetCharacterMovement _player2_2) "MOVE_Walking" 0))))))))))

(event EventBeginPlay
  (Utilities|Time|SetTimerbyFunctionName 0 "UpdateRope" 0.025 true true))

(fn ConstructionScript
  (bind _ropemesh (Variables|Default|GetRopeMesh))
  (bind _returnvalue (StaticMesh|GetBoundingBox _ropemesh))
  (bind (_min _max) (Utilities|Struct|BreakBox _returnvalue))
  (Components|StaticMesh|SetStaticMesh (Variables|Default|GetInstancedStaticMesh) (Variables|Default|GetRopeMesh))
  (Variables|Default|SetSpacing (+ (.Z (Math|Vector|BreakVector (- _max _min))) (Variables|Default|GetOffset))))

(fn OnRepPlayer2)

(fn OnRepPlayer1)

(fn AddSplineMesh
  (bind _spacing (Variables|Default|GetSpacing))
  (Components|InstancedStaticMesh|ClearInstances (Variables|Default|GetInstancedStaticMesh))
  (bind _output_get (LocalVariables|SetNumInstances (Math|Float|Floor (/ (Spline|GetSplineLength (Variables|Default|GetSpline)) (Variables|Default|GetSpacing)))))
  (for _index (range 0 _output_get)
    (Components|InstancedStaticMesh|AddInstance (Variables|Default|GetInstancedStaticMesh) (Math|Transform|MakeTransform (CallFunction|GetLocationatIndexLocal _index _spacing) (Math|Rotator|MakeRotfromZ (- (CallFunction|GetLocationatIndexLocal (+ _index 1) _spacing) (CallFunction|GetLocationatIndexLocal _index _spacing)))) false)))

(fn SetSplinePoints
  (bind (_sag _distance _p1location _p2location) (CallFunction|GetPlayerLocationsandDistance))
  (Spline|ClearSplinePoints (Variables|Default|GetSpline) false)
  (Spline|AddSplinePoint (Variables|Default|GetSpline) (.P2Location (CallFunction|GetPlayerLocationsandDistance)) "World" false)
  (Spline|AddSplinePoint (Variables|Default|GetSpline) (CallFunction|GetMiddlePoint _p1location _p2location _sag) "World" false)
  (Spline|AddSplinePoint (Variables|Default|GetSpline) (.P1Location (CallFunction|GetPlayerLocationsandDistance)) "World" false)
  (for _index (range 0 (- (Spline|GetNumberOfSplinePoints (Variables|Default|GetSpline)) 1))
    (Spline|SetSplinePointType (Variables|Default|GetSpline) _index "Curve" true)))

(fn GetLocationatIndexLocal
  (params (A :type Integer) (Spacing :type Float%20%28double-precision%29))
  (return (Spline|GetLocationatDistanceAlongSpline (Variables|Default|GetSpline) (* A Spacing) "Local")))

(fn ArePlayersValid
  (return (and (Utilities|IsValid (Variables|Default|GetPlayer1)) (Utilities|IsValid (Variables|Default|GetPlayer2)))))

(fn GetPlayerLocationsandDistance
  (bind _player1 (Variables|Default|GetPlayer1))
  (bind _player2 (Variables|Default|GetPlayer2))
  (bind _mesh (Variables|/Script/Engine.Character|GetMesh _player2))
  (bind _mesh_2 (Variables|/Script/Engine.Character|GetMesh _player1))
  (bind _returnvalue (Transformation|GetSocketLocation _mesh_2 "Hips"))
  (bind _returnvalue_2 (Transformation|GetSocketLocation _mesh "Hips"))
  (bind _returnvalue_3 (Math|Vector|Distance(Vector) _returnvalue _returnvalue_2))
  (return (Math|Float|Clamp(Float) (* (/ (Variables|Default|GetMaxLength) _returnvalue_3) (Variables|Default|GetSagMultiplier)) 0.0 (Variables|Default|GetMaxSag)) _returnvalue_3 _returnvalue _returnvalue_2))

(fn GetMiddlePoint
  (params (A :type Vector) (B :type Vector) (Sag :type Float%20%28double-precision%29))
  (return (- (/ (+ A B) 2.0) (Math|Vector|MakeVector 0.0 0.0 Sag))))

(fn GetLocationatIndexWorld
  (params (A :type Integer) (Spacing :type Float%20%28double-precision%29))
  (return (Spline|GetLocationatDistanceAlongSpline (Variables|Default|GetSpline) (* A Spacing) "World")))