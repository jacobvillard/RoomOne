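; Rope prototype actor that probes obstacles between player characters 0 and 1, drawing only debug visuals.
; Each server tick, it traces both ways between the players to find two hit points and their midpoint.
; It then traces inward to that midpoint from points on a horizontal circle of radius Offset, marking starts and hits.
; The angle step comes from NumOfSamples, but the loop count derives from that step, not the sample count.
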(event EventTick
  (params (DeltaSeconds :type Float%20%28single-precision%29))
  (bind _returnvalue (Game|GetPlayerCharacter 1))
  (bind _returnvalue_2 (Game|GetPlayerCharacter 0))
  (bind _returnvalue_3 (Transformation|GetActorLocation _returnvalue))
  (bind _returnvalue_4 (Transformation|GetActorLocation _returnvalue_2))
  ;[0.15 0.15 0.15 0.5] In and out
  (Networking|SwitchHasAuthority
    (:Authority
      (bind _outhit (Collision|LineTraceByChannel _returnvalue_4 _returnvalue_3 "TraceTypeQuery1" false 0 "ForOneFrame"))
      (bind _output_get (Variables|Default|SetHitNode1 (.Location (Collision|BreakHitResult _outhit))))
      (Rendering|Debug|DrawDebugPoint _output_get 5e+01 "(R=1.000000,G=0.000000,B=0.706903,A=1.000000)" 5.0)
      (bind _outhit_2 (Collision|LineTraceByChannel _returnvalue_3 _returnvalue_4 "TraceTypeQuery1" false 0 "ForOneFrame"))
      (bind _output_get_2 (Variables|Default|SetHitNode2 (.Location (Collision|BreakHitResult _outhit_2))))
      (Rendering|Debug|DrawDebugPoint _output_get_2 5e+01 "(R=1.000000,G=0.997643,B=0.000000,A=1.000000)" 5.0)
      ;[0.15 0.15 0.15 0.5] Circle of Points calculation
      (Variables|Default|SetMidpoint (/ (+ (Variables|Default|GetHitNode1) (Variables|Default|GetHitNode2)) 2.0))
      (Variables|Default|SetAnglestep (/ 3.6e+02 (Variables|Default|GetNumOfSamples)))
      (for _index (range 0 (Math|Float|Truncate (- (Variables|Default|GetAnglestep) 1.0)))
        (bind _output_get_3 (Variables|Default|SetAngleDegrees (* _index (Variables|Default|GetAnglestep))))
        (bind _output_get_4 (Variables|Default|SetAngleRadians (Math|Trig|DegreesToRadians _output_get_3)))
        (bind _output_get_5 (Variables|Default|SetOffsetVector (* (Math|Vector|Normalize (Math|Vector|MakeVector (Math|Trig|Cos(Radians) _output_get_4) (Math|Trig|Sin(Radians) _output_get_4) 0.0)) (Variables|Default|GetOffset))))
        (bind _output_get_6 (Variables|Default|SetSamplePoint (+ _output_get_5 (Variables|Default|GetMidpoint))))
        (bind _outhit_3 (Collision|LineTraceByChannel _output_get_6 (Variables|Default|GetMidpoint) "TraceTypeQuery1" false 0 "ForOneFrame"))
        (Rendering|Debug|DrawDebugPoint (.Location (Collision|BreakHitResult _outhit_3)) 5e+01 "(R=0.000000,G=0.021426,B=0.296875,A=1.000000)" 5.0)
        (Rendering|Debug|DrawDebugPoint (.TraceStart (Collision|BreakHitResult _outhit_3)) 5e+01 "(R=0.888773,G=0.858318,B=1.000000,A=1.000000)" 5.0)))))

(fn ConstructionScript)