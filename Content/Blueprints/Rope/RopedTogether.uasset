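; Rope actor that tethers the first two third-person characters, launching them toward each other when its spline exceeds MaxLength.
; Server-only timers rebuild the spline between both players through stored bend points and lay instanced rope meshes along it.
; A slower timer sphere-traces along the spline to add obstacle bends, resetting to a sagging midpoint when none are found.
; Spline-mesh, cable-attachment and bone-rope variants remain as unused functions, alongside debug prints.
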(event Custom|Debug
  (Networking|SwitchHasAuthority
    (:Authority
      (Development|PrintString (Utilities|String|ToString(Integer) (Utilities|Array|Length (Variables|Default|GetSplinePoints))) true true "(R=0.000000,G=0.660000,B=1.000000,A=1.000000)" 1.0))))

(event Custom|UpdateRope
  (bind (_sag _distance _p1location _p2location) (CallFunction|GetPlayerLocationsandDistance))
  (bind _pullforce (Variables|Default|GetPullForce))
  (bind _returnvalue (Math|Vector|GetUnitDirection(Vector) _p1location _p2location))
  (bind _returnvalue_2 (* _returnvalue _pullforce))
  (if (CallFunction|ArePlayersValid)
    (Networking|SwitchHasAuthority
      (:Authority
        (CallFunction|SetSplinePoints)
        (CallFunction|AddSplineMesh)
        (Networking|SwitchHasAuthority
          (:Authority
            (if (> (Spline|GetSplineLength (Variables|Default|GetSpline)) (Variables|Default|GetMaxLength))
              (Character|LaunchCharacter (Variables|Default|GetPlayer1) _returnvalue_2 true true)
              (Character|LaunchCharacter (Variables|Default|GetPlayer2) (* _returnvalue_2 -1.0) true true))))))))

(event Custom|SplineColliders
  (CallFunction|AddSplineColliders))

(event EventBeginPlay
  (Utilities|Time|SetTimerbyEvent (delegate Custom|Debug) 1.0 true)
  (Variables|/Script/CableComponent.CableComponent|SetCableLength (Variables|Default|GetCable) (Variables|Default|GetMaxLength))
  (Utilities|FlowControl|Delay 2.0)
  (Networking|SwitchHasAuthority
    (:Authority
      (bind _outactors (Actor|GetAllActorsOfClass "/Game/ThirdPerson/Blueprints/BP_ThirdPersonCharacter.BP_ThirdPersonCharacter_C"))
      (bind _output_get (Variables|Default|SetPlayers _outactors))
      (Variables|Default|SetPlayer1 (Utilities|Array|Get(acopy) _output_get))
      (Variables|Default|SetPlayer2 (Utilities|Array|Get(acopy) _output_get 1))
      (Utilities|Time|SetTimerbyFunctionName 0 "UpdateRope" 0.025 true)
      (Utilities|Time|SetTimerbyFunctionName 0 "SplineColliders" 0.05 true))))

(event Input|KeyboardEvents|DebugKeyT
  (params (Key :type Key%20Structure :default "None") (ActionValue :type Input%20Action%20Value%20Structure))
  (bind _spline (Variables|Default|GetSpline))
  (:Pressed
    (Development|PrintString (Utilities|String|ToString(Vector) (Transformation|GetActorLocation (Variables|Default|GetPlayer1))) true true "(R=0.000000,G=0.660000,B=1.000000,A=1.000000)" 5.0)
    (Development|PrintString (Utilities|String|ToString(Vector) (Transformation|GetActorLocation (Variables|Default|GetPlayer2))) true true "(R=0.000000,G=0.660000,B=1.000000,A=1.000000)" 5.0)
    (for _index (range 0 (- (Spline|GetNumberOfSplinePoints _spline) 1))
      (Development|PrintString (Utilities|String|Append (Utilities|String|ToString(Vector) (.position (Spline|GetSplinePointAt _spline _index "World"))) "SplinePoint") true true "(R=0.000000,G=0.660000,B=1.000000,A=1.000000)" 5.0))))

(fn ConstructionScript
  (bind _ropemesh (Variables|Default|GetRopeMesh))
  (bind _returnvalue (StaticMesh|GetBoundingBox _ropemesh))
  (bind (_min _max) (Utilities|Struct|BreakBox _returnvalue))
  (Components|StaticMesh|SetStaticMesh (Variables|Default|GetInstancedStaticMesh) (Variables|Default|GetRopeMesh))
  (Variables|Default|SetSpacing (+ (.Z (Math|Vector|BreakVector (- _max _min))) (Variables|Default|GetOffset))))

(fn OnRepPlayer2)

(fn OnRepPlayer1)

(fn TraceforObstacle
  (bind (_sag _distance _p1location _p2location) (CallFunction|GetPlayerLocationsandDistance))
  (Utilities|Array|Clear (Variables|Default|GetTemporarySplinePoints))
  (Utilities|Array|Add (Variables|Default|GetTemporarySplinePoints) (CallFunction|GetMiddlePoint _p1location _p2location _sag))
  (Variables|Default|SetTraceStartLocation _p1location))

(fn AddSplineMesh
  (bind _spacing (Variables|Default|GetSpacing))
  (Components|InstancedStaticMesh|ClearInstances (Variables|Default|GetInstancedStaticMesh))
  (bind _output_get (LocalVariables|SetNumInstances (Math|Float|Floor (/ (Spline|GetSplineLength (Variables|Default|GetSpline)) (Variables|Default|GetSpacing)))))
  (for _index (range 0 _output_get)
    (Components|InstancedStaticMesh|AddInstance (Variables|Default|GetInstancedStaticMesh) (Math|Transform|MakeTransform (CallFunction|GetLocationatIndexLocal _index _spacing) (Math|Rotator|MakeRotfromZ (- (CallFunction|GetLocationatIndexLocal (+ _index 1) _spacing) (CallFunction|GetLocationatIndexLocal _index _spacing)))) false)))

(fn SetSplinePoints
  (bind (_sag _distance _p1location _p2location) (CallFunction|GetPlayerLocationsandDistance))
  (bind _spline (Variables|Default|GetSpline))
  (Spline|ClearSplinePoints (Variables|Default|GetSpline) false)
  (Spline|AddSplinePoint (Variables|Default|GetSpline) _p1location "World" false)
  (for (_array_element _array_index) (Variables|Default|GetSplinePoints)
    (Spline|AddSplinePoint (Variables|Default|GetSpline) (.Position (Utilities|Struct|BreakSplinePoint _array_element)) "World" true)
    (Spline|SetTangentsatSplinePoint _spline (+ _array_index 1) (.ArriveTangent (Utilities|Struct|BreakSplinePoint _array_element)) (.LeaveTangent (Utilities|Struct|BreakSplinePoint _array_element)) "World" false)
    (Spline|SetRotationatSplinePoint _spline (+ _array_index 1) (.Rotation (Utilities|Struct|BreakSplinePoint _array_element)) "World" false))
  (Spline|AddSplinePoint (Variables|Default|GetSpline) _p2location "World" false)
  (for _index (range 0 (- (Spline|GetNumberOfSplinePoints (Variables|Default|GetSpline)) 1))
    (Spline|SetSplinePointType (Variables|Default|GetSpline) _index "Curve" true)))

(fn GetLocationatIndexLocal
  (params (A :type Integer) (Spacing :type Float%20%28double-precision%29))
  (return (Spline|GetLocationatDistanceAlongSpline (Variables|Default|GetSpline) (* A Spacing) "Local")))

(fn UnusedMeshonSpline
  (bind _splinemesh (Variables|Unused|GetSplineMesh))
  (for _array_element _splinemesh
    (Components|DestroyComponent _array_element))
  (Utilities|Array|Clear _splinemesh)
  (for _index (range 0 (- (Spline|GetNumberOfSplinePoints (Variables|Default|GetSpline)) 2))
    (bind _returnvalue (AddComponent|AddSplineMeshComponent false))
    (Transformation|SetMobility _returnvalue "Movable")
    (SplineMesh|SetStartandEnd _returnvalue (.Location (Spline|GetLocationandTangentatSplinePoint (Variables|Default|GetSpline) _index "Local")) (.Tangent (Spline|GetLocationandTangentatSplinePoint (Variables|Default|GetSpline) _index "Local")) (.Location (Spline|GetLocationandTangentatSplinePoint (Variables|Default|GetSpline) (- _index -1) "Local")) (.Tangent (Spline|GetLocationandTangentatSplinePoint (Variables|Default|GetSpline) (- _index -1) "Local")) false :!class /Script/Engine.SplineMeshComponent)
    (SplineMesh|SetForwardAxis _returnvalue "Z" false)
    (Components|StaticMesh|SetStaticMesh _returnvalue (Variables|Default|GetRopeMesh))
    (Utilities|Array|Add (Variables|Unused|GetSplineMesh) _returnvalue)))

(fn UnusedCableAttachment
  (Transformation|AttachActorToActor (Variables|Default|GetPlayer1) "None" "SnapToTarget" "SnapToTarget" "KeepRelative" true)
  (Class|CableComponent|SetAttachEndto (Variables|Default|GetCable) (Variables|Default|GetPlayer2) "None" "None"))

(fn UnusedBoneRope
  (bind _asrope_anim (Utilities|Casting|CastToRopeAnim (Components|SkeletalMesh|GetAnimInstance (Variables|Default|GetSkeletalMesh))))
  (bind _output_get (Variables|Unused|SetAs%20Rope%20Anim _asrope_anim))
  (Variables|/Game/Blueprints/Rope/RopeAnim.RopeAnim_C|SetSplineComponent _output_get (Variables|Default|GetSpline)))

(fn ArePlayersValid
  (return (and (Utilities|IsValid (Variables|Default|GetPlayer1)) (Utilities|IsValid (Variables|Default|GetPlayer2)))))

(fn GetPlayerLocationsandDistance
  (bind _player1 (Variables|Default|GetPlayer1))
  (bind _player2 (Variables|Default|GetPlayer2))
  (bind _returnvalue (Transformation|GetActorLocation _player2))
  (bind _returnvalue_2 (Transformation|GetActorLocation _player1))
  (bind _returnvalue_3 (Math|Vector|Distance(Vector) _returnvalue_2 _returnvalue))
  (return (Math|Float|Clamp(Float) (* (/ (Variables|Default|GetMaxLength) _returnvalue_3) (Variables|Default|GetSagMultiplier)) 0.0 (Variables|Default|GetMaxSag)) _returnvalue_3 _returnvalue_2 _returnvalue))

(fn GetMiddlePoint
  (params (A :type Vector) (B :type Vector) (Sag :type Float%20%28double-precision%29))
  (return (- (/ (+ A B) 2.0) (Math|Vector|MakeVector 0.0 0.0 Sag))))

(fn AddSplineColliders
  (bind _p1location (CallFunction|GetPlayerLocationsandDistance))
  (bind (_sag _distance _p1location_2 _p2location) (CallFunction|GetPlayerLocationsandDistance))
  (bind _tracespacing (Variables|Default|GetTraceSpacing))
  (bind _splinepoints (Variables|Default|GetSplinePoints))
  (bind _splinepoints_2 (Variables|Default|GetSplinePoints))
  (bind _returnvalue (Math|Vector|GetUnitDirection(Vector) _p1location_2 _p2location))
  (bind _returnvalue_2 (* _tracespacing 1e+01))
  (Variables|Default|SetAnyHit false)
  (bind _output_get (Variables|Default|SetColliderCount (Math|Float|Floor (/ (Spline|GetSplineLength (Variables|Default|GetSpline)) (Variables|Default|GetTraceSpacing)))))
  (for _index (range 0 _output_get)
    (bind (_outhit _returnvalue_3) (Collision|SphereTraceByChannel (.location (Math|Transform|MakeTransform (CallFunction|GetLocationatIndexWorld _index _returnvalue_2) (Math|Rotator|MakeRotfromZ (- (CallFunction|GetLocationatIndexWorld (+ _index 1) _returnvalue_2) (CallFunction|GetLocationatIndexWorld _index _returnvalue_2))))) (.location (Math|Transform|MakeTransform (CallFunction|GetLocationatIndexWorld _index _returnvalue_2) (Math|Rotator|MakeRotfromZ (- (CallFunction|GetLocationatIndexWorld (+ _index 1) _returnvalue_2) (CallFunction|GetLocationatIndexWorld _index _returnvalue_2))))) (Variables|Default|GetSphereRadius) "TraceTypeQuery1" false (Variables|Default|GetPlayers) "ForOneFrame" true "(R=1.000000,G=0.000000,B=0.000000,A=1.000000)" "(R=0.000000,G=1.000000,B=0.000000,A=1.000000)" 0.05))
    (if _returnvalue_3
      (Variables|Default|SetHit%20Actor (.HitActor (Collision|BreakHitResult _outhit)))
      (Variables|Default|SetTrace%20Start (.TraceStart (Collision|BreakHitResult _outhit)))
      (bind _output_get_2 (Variables|Default|SetHitLocation (.TraceStart (Collision|BreakHitResult _outhit))))
      (Variables|Default|SetSpline%20Point (Utilities|Struct|MakeSplinePoint 0.0 _output_get_2 (Math|Vector|GetUnitDirection(Vector) (.TraceStart (Collision|BreakHitResult _outhit)) _p1location) (* (Math|Vector|GetUnitDirection(Vector) (.TraceStart (Collision|BreakHitResult _outhit)) _p1location) -1.0) (Math|Rotator|FindLookatRotation _p1location (.TraceStart (Collision|BreakHitResult _outhit)))))
      (Variables|Default|SetCanAddPoint false)
      (for _array_element (Variables|Default|GetSplinePoints)
        (Variables|Default|SetCanAddPoint (< (Math|Vector|Distance(Vector) (.Position (Utilities|Struct|BreakSplinePoint _array_element)) (Variables|Default|GetHitLocation)) (Variables|Default|GetDistanceThreshold))))
      (if (not (Variables|Default|GetCanAddPoint))
        (if (< (Utilities|Array|Length (Variables|Default|GetSplinePoints)) (Variables|Default|GetMaxBends))
          (bind _returnvalue_4 (Game|AddComponentbyClass "/Script/Engine.SphereComponent" false (Math|Transform|MakeTransform (Variables|Default|GetHitLocation) "0, 0, 0" "1.000000,1.000000,1.000000")))
          (bind _output_get_3 (Variables|Default|SetPointSphere _returnvalue_4))
          (Components|Sphere|SetSphereRadius _output_get_3 (Variables|Default|GetSphereRadius) true)
          (if (not (Collision|IsOverlappingActor _returnvalue_4 (Variables|Default|GetHit%20Actor) :!class /Script/Engine.PrimitiveComponent))
            (bind _output_get_4 (Variables|Default|SetSpline%20Point (Utilities|Struct|MakeSplinePoint 0.0 (+ (* (Math|Vector|GetUnitDirection(Vector) (.Origin (Collision|GetActorBounds (Variables|Default|GetHit%20Actor) false false)) (Variables|Default|GetTrace%20Start)) 5.0) (Variables|Default|GetTrace%20Start)) (.ArriveTangent (Utilities|Struct|BreakSplinePoint (Variables|Default|GetSpline%20Point))) (.LeaveTangent (Utilities|Struct|BreakSplinePoint (Variables|Default|GetSpline%20Point))) (.Rotation (Utilities|Struct|BreakSplinePoint (Variables|Default|GetSpline%20Point))))))
            (Utilities|Array|Add _splinepoints _output_get_4)
            (Variables|Default|SetAnyHit true)
            (bind _returnvalue_5 (Collision|LineTraceComponent (Variables|Default|GetPointSphere) (.Position (Utilities|Struct|BreakSplinePoint (Utilities|Array|Get(acopy) _splinepoints (- (Utilities|Array|Length _splinepoints) 1)))) (.P1Location (CallFunction|GetPlayerLocationsandDistance)) false false false))
            (Components|DestroyComponent (Variables|Default|GetPointSphere))
            (if _returnvalue_5
              (Utilities|Array|RemoveIndex _splinepoints_2 (- (Utilities|Array|Length _splinepoints_2) 1))))))
      (elif (not (Variables|Default|GetAnyHit))
        (Utilities|Array|Clear (Variables|Default|GetSplinePoints))
        (Utilities|Array|Add (Variables|Default|GetSplinePoints) (Utilities|Struct|MakeSplinePoint 0.5 (CallFunction|GetMiddlePoint _p1location_2 _p2location _sag) (* _returnvalue -1.0) _returnvalue (Math|Rotator|FindLookatRotation _p1location_2 _p2location)))))))

(fn GetLocationatIndexWorld
  (params (A :type Integer) (Spacing :type Float%20%28double-precision%29))
  (return (Spline|GetLocationatDistanceAlongSpline (Variables|Default|GetSpline) (* A Spacing) "World")))