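; AC_ChatPC is a player controller component that runs the text chat system.
; On BeginPlay it creates the chat widget for the local controller and caches its chat box, which Enter focuses and PageUp/PageDown scroll.
; SendChatMessage relays text through every PlayerArray controller's component to AddChatMessageOnOwningClient, passing the sender's array index.
; MulticastSystemMessage posts "[System]:" prefixed messages wherever the chat box is valid.
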(event Custom|SendChatMessage
  (params (Message :type String) (SenderIndex :type Player%20Controller%20Object%20Reference))
  (bind _returnvalue (Game|GetGameState))
  (bind _playerarray (Variables|/Script/Engine.GameStateBase|GetPlayerArray _returnvalue))
  ;[0.15 0.15 0.15 0.5] Broadcasts Player Messages to Everyone
  (for _array_element _playerarray
    (CallFunction|AddChatMessageonOwningClient (Actor|GetComponentbyClass (Game|GetPlayerController _array_element) "AC_ChatPC_C") Message (Utilities|Array|FindItem _playerarray (Variables|/Script/Engine.Controller|GetPlayerState SenderIndex)))))

(event Custom|AddChatMessageOnOwningClient
  (params (Message :type String) (SenderIndex :type Integer))
  ;[0.15 0.15 0.15 0.5] Adds Player Messages to Owning Client
  (Default|AddChatMessage (Variables|Default|GetChatBoxRef) Message false SenderIndex))

(event Custom|MulticastSystemMessage
  (params (Message :type String))
  ;[0.15 0.15 0.15 0.5] System Wide Message
  (if (Utilities|IsValid (Variables|Default|GetChatBoxRef))
    (Default|AddChatMessage (Variables|Default|GetChatBoxRef) (Utilities|String|Append "[System]: " Message) true)))

(event EventBeginPlay
  ;[0.15 0.15 0.15 0.5] Create Chat UI Widget, Sets ChatUI and ChatBox References
  (bind _asplayer_controller (Utilities|Casting|CastToPlayerController (Components|GetOwner)))
  (if (Pawn|IsLocalPlayerController _asplayer_controller)
    (bind _returnvalue (UserInterface|CreateWidget "/Game/Blueprints/Systems/Chat/WB_ChatUI.WB_ChatUI_C"))
    (bind _output_get (Variables|Default|SetChatUIRef _returnvalue))
    (UserInterface|Viewport|AddtoViewport _output_get 0)
    (Variables|Default|SetChatBoxRef (Variables|/Game/Blueprints/Systems/Chat/WB_ChatUI.WB_ChatUI_C|GetWB_ChatBox _output_get))))

(event Input|KeyboardEvents|Enter
  (params (Key :type Key%20Structure :default "None"))
  ;[0.15 0.15 0.15 0.5] Chat Keybinds and Input
  ;;[0.15 0.15 0.15 0.5] Toggle Chat
  (:Pressed
    (Default|ShowChat (Variables|Default|GetChatUIRef))
    (Default|FocusChat (Variables|Default|GetChatBoxRef))))

(event Input|KeyboardEvents|PageUp
  (params (Key :type Key%20Structure :default "None"))
  ;[0.15 0.15 0.15 0.5] Chat Keybinds and Input
  ;;[0.15 0.15 0.15 0.5] Scroll Chat
  (:Pressed
    (Default|Scroll (Variables|Default|GetChatBoxRef) true)))

(event Input|KeyboardEvents|PageDown
  (params (Key :type Key%20Structure :default "None"))
  ;[0.15 0.15 0.15 0.5] Chat Keybinds and Input
  ;;[0.15 0.15 0.15 0.5] Scroll Chat
  (:Pressed
    (Default|Scroll (Variables|Default|GetChatBoxRef) false)))