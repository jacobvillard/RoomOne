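; Train pawn that drives itself along the spline of its ActivePath.
; Each tick it adds forward movement input scaled by Speed, then GetPath turns it to face the spline.
; Steering projects a short look-ahead along the nearest tangent back onto the spline and looks at that point.
; Rotation updates stop near the spline's end or without a valid path, while forward input continues.
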(event EventBeginPlay)

(event Collision|EventActorBeginOverlap
  (params (OtherActor :type Actor%20Object%20Reference)))

(event EventTick
  (params (DeltaSeconds :type Float%20%28single-precision%29))
  (Pawn|Input|AddMovementInput (Transformation|GetActorForwardVector) (Variables|Default|GetSpeed) false)
  (CallFunction|GetPath))

(fn ConstructionScript)

(fn GetPath
  (bind _returnvalue (Transformation|GetActorLocation))
  (bind _activepath (Variables|Default|GetActivePath))
  (bind _spline (Variables|/Game/Blueprints/Train/Path.Path_C|GetSpline _activepath))
  (Utilities|IsValid _activepath
    (:Is%20Valid
      (if (not (Utilities|Operators|EqualEqual (Spline|GetLocationatSplinePoint _spline (Spline|GetNumberOfSplinePoints _spline) "World") _returnvalue 5e+01))
        (Transformation|SetActorRotation (Math|Rotator|FindLookatRotation _returnvalue (Spline|FindLocationClosesttoWorldLocation _spline (+ (* (Math|Vector|Normalize (Class|SplineComponent|FindTangentClosesttoWorldLocation _spline _returnvalue "World")) 5e+01) _returnvalue) "World")))))))