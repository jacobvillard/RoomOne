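; BP_Enabler is an overlap trigger that reveals hidden platforms when a locally controlled third-person character enters it.
; Its construction script caches every BP_Platform carrying the TargetTag into an Actors array.
; On begin overlap, it casts to BP_ThirdPersonCharacter, checks that its controller is local, then unhides each cached platform, with no logic to hide them again.
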(event Collision|EventActorBeginOverlap
  (params (OtherActor :type Actor%20Object%20Reference))
  ;[0.15 0.15 0.15 0.5] Unhide Actors if Local Controller
  (bind _asbp_third_person_character (Utilities|Casting|CastToBP_ThirdPersonCharacter OtherActor))
  (if (Pawn|IsLocalController (Pawn|GetController _asbp_third_person_character))
    (for _array_element (Variables|Default|GetActors)
      (Rendering|SetActorHiddenInGame _array_element false))))

(fn ConstructionScript
  ;[0.15 0.15 0.15 0.5] Get Tagged Actors
  (bind _outactors (Actor|GetAllActorsOfClasswithTag "/Game/Invisible/BP_Platform.BP_Platform_C" (Variables|Default|GetTargetTag)))
  (Variables|Default|SetActors _outactors))