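; Arrow Assault enemy: an animated gargoyle that fires arrow projectiles from its FirePoint on a looping timer, with the interval randomised once at BeginPlay.
; When targeting is enabled, a second fast timer re-picks a random third-person character each tick and turns the enemy toward it with RInterpTo.
; Player input is enabled so the F key can trigger a damage test.
; Death simply destroys the actor.
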(event Custom|Event%20RotateToTarget
  ;[0.15 0.15 0.15 0.5] Finds Target's current location and updates Enemy Rotation to match.
  (Transformation|SetActorRotation (Math|Interpolation|RInterpTo (Transformation|GetActorRotation) (Math|Rotator|FindLookatRotation (Transformation|GetActorLocation) (Transformation|GetActorLocation (Variables|Default|GetTarget))) (Utilities|Time|GetWorldDeltaSeconds) 5e+02)))

(event Custom|Shoot
  ;[0.15 0.15 0.15 0.5] Spawns set projectile at set frequency in the direction the Enemy BP is facing
  (Game|SpawnActorfromClass "/Game/Level/ArrowAssault/BP_BaseProjectile_Child_Arrow.BP_BaseProjectile_Child_Arrow_C" (Transformation|GetWorldTransform (Variables|Default|GetFirePoint)) "Undefined" "MultiplyWithRoot" self 1e+03 0.0 true 25.0 0))

(event Custom|PickTarget
  ;[0.15 0.15 0.15 0.5] Randomly sets a player as the target if Targeting is Enabled
  (if (Variables|Default|GetTargetingEnabled)
    (bind _outactors (Actor|GetAllActorsOfClass "/Game/Blueprints/Characters/Goblin/BP_ThirdPersonCharacter.BP_ThirdPersonCharacter_C"))
    (Variables|Default|SetTarget (.OutItem (Utilities|Array|Random _outactors)))
    (CallFunction|EventRotatetoTarget)))

(event EventBeginPlay
  (Components|Animation|PlayAnimation (Variables|Default|GetSkeletalMesh) "/Game/Level/AlexiAssets/202507211307_MetalGargoyle.202507211307_MetalGargoyle" true)
  ;[0.15 0.15 0.15 0.5] For testing Damage and Health logic
  ;;[0.15 0.15 0.15 0.5] Enables Player input
  (Input|EnableInput (Game|GetPlayerController 0))
  ;[0.15 0.15 0.15 0.5] Spawns set projectile at set frequency in the direction the Enemy BP is facing
  (Utilities|Time|SetTimerbyEvent (delegate Custom|Shoot) (Math|Random|RandomFloatinRange (Variables|Projectiles|GetFrequencyMin) (Variables|Projectiles|GetFrequencyMax)) true)
  ;[0.15 0.15 0.15 0.5] Updates enemy rotation every 0.1 seconds
  (Utilities|Time|SetTimerbyEvent (delegate Custom|PickTarget) 0.1 true))

(event Input|KeyboardEvents|F
  (params (Key :type Key%20Structure))
  ;[0.15 0.15 0.15 0.5] For testing Damage and Health logic
  ;;[0.15 0.15 0.15 0.5] When the user presses F, applies damage
  (:Pressed
    (Development|PrintString "Pressed F")
    (Game|Damage|ApplyDamage 0 25.0 0 0)))

(fn ConstructionScript)

(fn Death
  (Actor|DestroyActor))