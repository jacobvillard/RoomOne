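; BP_MasterCharacter is an Arrow Assault character Blueprint that manages health, damage and a health bar widget.
; Health starts at MaxHealth; AnyDamage subtracts damage, updates the WBP_HealthBar percentage and checks for death.
; Each hit toggles the bar's visibility, then toggles it again after a short Delay, rather than explicitly showing and hiding it.
; Death is a placeholder that only prints a message.
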(event Custom|ActorHealthChanged
  ;[0.15 0.15 0.15 0.5] Shows Enemy health bar widget for 2 seconds, before hiding again
  (CallFunction|ToggleHealthBar)
  (Utilities|FlowControl|Delay 2.0)
  (CallFunction|ToggleHealthBar))

(event Game|Damage|EventAnyDamage
  (params (Damage :type Float%20%28single-precision%29) (DamageType :type Damage%20Type%20Object%20Reference) (InstigatedBy :type Controller%20Object%20Reference) (DamageCauser :type Actor%20Object%20Reference))
  ;[0.15 0.15 0.15 0.5] Displays and Updates Health
  (CallFunction|ActorHealthChanged)
  (Variables|Health|SetHealth (- (Variables|Health|GetHealth) Damage))
  (CallFunction|UpdateHealthBar)
  (CallFunction|CheckHealth))

(event EventBeginPlay
  ;[0.15 0.15 0.15 0.5] Sets health to Max health on Play
  (Variables|Health|SetHealth (Variables|Health|GetMaxHealth)))

(fn ConstructionScript)

(fn ToggleHealthBar
  ;[0.15 0.15 0.15 0.5] If health isn't visible, set to visible in both the boolean and the component and vice versa.
  (if (not (Variables|Health|GetHealthVisible))
    (Variables|Health|SetHealthVisible true)
    (Rendering|SetVisibility (Variables|Default|GetHealthBarWidget) true false)
    (else
      (Variables|Health|SetHealthVisible false)
      (Rendering|SetVisibility (Variables|Default|GetHealthBarWidget) false false))))

(fn UpdateHealthBar
  (bind _aswbp_health_bar (Utilities|Casting|CastToWBP_HealthBar (UserInterface|GetUserWidgetObject (Variables|Default|GetHealthBarWidget)))
    (:then
      (Progress|SetPercent (Variables|/Game/Level/ArrowAssault/WBP_HealthBar.WBP_HealthBar_C|GetHealthBar _aswbp_health_bar) (/ (Variables|Health|GetHealth) (Variables|Health|GetMaxHealth))))
    (:CastFailed
      (Development|PrintString "Cast Failed"))))

(fn CheckHealth
  (if (<= (Variables|Health|GetHealth) 0.0)
    ;[0.15 0.15 0.15 0.5] Death Logic
    (CallFunction|Death)))

(fn Death
  ;[0.15 0.15 0.15 0.5] Does nothing. For now.
  (Development|PrintString "Player Died"))