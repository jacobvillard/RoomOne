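; BP_DoorWay2 is a ball-run level doorway with two trap obstacles and arches that break when a Ball hits them.
; SetTrap disables collision on the selected obstacle, while overlapping either obstacle calls TriggerRagdoll on the third-person character.
; A Ball overlap destroys the intact arches, reveals a physics-simulated broken version and activates Gems.
; The Gems activation event switches four static meshes to simulated physics with physics-only collision.
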(event OnComponentBeginOverlap(Obstacle1)
  (params (OverlappedComponent :type Primitive%20Component%20Object%20Reference) (OtherActor :type Actor%20Object%20Reference) (OtherComp :type Primitive%20Component%20Object%20Reference) (OtherBodyIndex :type Integer) (bFromSweep :type Boolean) (SweepResult :type Hit%20Result%20Structure%20%28by%20ref%29))
  (bind _asbp_third_person_character (Utilities|Casting|CastToBP_ThirdPersonCharacter OtherActor))
  (Default|TriggerRagdoll _asbp_third_person_character false))

(event OnComponentBeginOverlap(Obstacle0)
  (params (OverlappedComponent :type Primitive%20Component%20Object%20Reference) (OtherActor :type Actor%20Object%20Reference) (OtherComp :type Primitive%20Component%20Object%20Reference) (OtherBodyIndex :type Integer) (bFromSweep :type Boolean) (SweepResult :type Hit%20Result%20Structure%20%28by%20ref%29))
  (bind _asbp_third_person_character (Utilities|Casting|CastToBP_ThirdPersonCharacter OtherActor))
  (Default|TriggerRagdoll _asbp_third_person_character false))

(event OnComponentActivated(Gems)
  (params (Component :type Actor%20Component%20Object%20Reference) (bReset :type Boolean))
  (for _array_element (Utilities|Array|MakeArray (Variables|Default|GetStaticMesh1) (Variables|Default|GetStaticMesh) (Variables|Default|GetStaticMesh2) (Variables|Default|GetStaticMesh3))
    (Physics|SetSimulatePhysics _array_element true)
    (Collision|SetCollisionEnabled _array_element "PhysicsOnly")))

(event Custom|SetTrap
  (params (Selection :type Integer))
  (switch int Selection
    (:0
      (Collision|SetCollisionEnabled (Variables|Default|GetObstacle0) "NoCollision"))
    (:1
      (Collision|SetCollisionEnabled (Variables|Default|GetObstacle1) "NoCollision"))))

(event Collision|EventActorBeginOverlap
  (params (OtherActor :type Actor%20Object%20Reference))
  (bind _archesbroken (Variables|Default|GetArchesBroken))
  (Utilities|Casting|CastToBall OtherActor)
  (bind _arches (Variables|Default|GetArches)
    (:then
      (Components|DestroyComponent _arches)
      (Rendering|SetVisibility _archesbroken true false)
      (Physics|SetSimulatePhysics _archesbroken true)
      (Components|Activation|Activate (Variables|Default|GetGems) false))
    (:else)))

(fn ConstructionScript)