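; BP_RandomFloorTiling is a Ball Run floor actor that varies its look with randomly picked tile meshes.
; Its Construction Script gives each of the nine Floor mesh components an independent random pick from TilesArray, so tiles can repeat.
; The pick uses no seeded stream, so the layout can change whenever construction reruns.
; The event graph has no active logic.
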(event EventBeginPlay)

(event Collision|EventActorBeginOverlap
  (params (OtherActor :type Actor%20Object%20Reference)))

(event EventTick
  (params (DeltaSeconds :type Float%20%28single-precision%29)))

(fn ConstructionScript
  (for _array_element (Utilities|Array|MakeArray (Variables|Default|GetFloor1) (Variables|Default|GetFloor2) (Variables|Default|GetFloor3) (Variables|Default|GetFloor4) (Variables|Default|GetFloor5) (Variables|Default|GetFloor6) (Variables|Default|GetFloor7) (Variables|Default|GetFloor8) (Variables|Default|GetFloor9))
    (Components|StaticMesh|SetStaticMesh _array_element (.OutItem (Utilities|Array|Random (Variables|Default|GetTilesArray))))))