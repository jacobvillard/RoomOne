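; Bomb for the Bomb Tag mode, which reports pickups by overlapping characters, drops and its explosion to BP_BombTagManager.
; The manager's light event starts a fuse timeline scaled to the given time, dissolving the fuse material and moving sparks between sockets.
; At burnout it plays a sim-cached explosion, then swaps the mesh for a temporary BP_BombBreakable shattered by field strain and radial impulse.
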(event OnComponentBeginOverlap(Box)
  (params (OverlappedComponent :type Primitive%20Component%20Object%20Reference) (OtherActor :type Actor%20Object%20Reference) (OtherComp :type Primitive%20Component%20Object%20Reference) (OtherBodyIndex :type Integer) (bFromSweep :type Boolean) (SweepResult :type Hit%20Result%20Structure%20%28by%20ref%29))
  (bind _asbp_third_person_character (Utilities|Casting|CastToBP_ThirdPersonCharacter OtherActor))
  (CallFunction|ServerUpdateCurrentHolder _asbp_third_person_character))

(event Custom|LightFuse
  (params (FuseTimer :type Float%20%28double-precision%29))
  (bind _fuse (Variables|Default|GetFuse))
  (bind _returnvalue (Transformation|GetSocketTransform _fuse "FuseEnd" "RTS_World"))
  (Components|Timeline|SetPlayRate (Variables|Default|GetFuseTimeline) (/ 1.0 FuseTimer))
  (Components|Activation|Activate (Variables|Default|GetNS_FuseSparks) false)
  (Components|Animation|PlayAnimation (Variables|Default|GetFuse) "/Game/Art/Meshes/Internal/CustomMeshes/Bomb/FuseAnim.FuseAnim" true)
  (bind (_direction _burnamount _sparkposition) (Timeline|FuseTimeline Play)
    (:Update
      (Rendering|Material|SetScalarParameterValue (Variables|Default|GetFuseDMI) "DissolveAmount" _burnamount :!class /Script/Engine.MaterialInstanceDynamic)
      (Utilities|FlowControl|Sequence
        (:then_0
          (Transformation|SetWorldLocation (Variables|Default|GetNS_FuseSparks) (Math|Vector|Lerp(Vector) (.location _returnvalue) (.location (Transformation|GetSocketTransform (Variables|Default|GetFuse) "FuseBase" "RTS_World")) _sparkposition) false false))
        (:then_1
          (Transformation|SetWorldRotation (Variables|Default|GetNS_FuseSparks) (Math|Rotator|Lerp(Rotator) (.rotation _returnvalue) "0.000000,1.000000,0.000000" _sparkposition) false false))))
    (:Finished
      (Components|Activation|Deactivate (Variables|Default|GetNS_FuseSparks))
      (Utilities|Time|SetTimerbyEvent (delegate Custom|BreakBomb) 0.4)
      (Components|Activation|Activate (Variables|Default|GetBombExplosion) false)
      (Collision|SetCollisionEnabled (Variables|Default|GetStaticMesh) "NoCollision"))))

(event Custom|BreakBomb
  (Rendering|SetVisibility (Variables|Default|GetStaticMesh) false false)
  (bind _returnvalue (Game|SpawnActorfromClass "/Game/Level/BombTag/BP_BombBreakable.BP_BombBreakable_C" (Transformation|GetRelativeTransform (Variables|Default|GetStaticMesh)) "Undefined" "MultiplyWithRoot" 0 0))
  (Variables|Default|SetBreakableBomb _returnvalue)
  (bind _returnvalue_2 (AddComponent|AddRadialFalloff (Variables|Default|GetBreakableBomb)))
  (Class|FieldSystemComponent|ApplyPhysicsField (Variables|/Game/Level/BombTag/BP_BombBreakable.BP_BombBreakable_C|GetFieldSystem (Variables|Default|GetBreakableBomb)) true "Field_ExternalClusterStrain" 0 (Field|SetRadialFalloff _returnvalue_2 5e+05 0.0 1.0 0.0 2e+02 (Transformation|GetWorldLocation (Variables|Default|GetStaticMesh)) "Field_FallOff_None"))
  (Physics|AddRadialImpulse (Variables|/Game/Level/BombTag/BP_BombBreakable.BP_BombBreakable_C|GetGeometryCollection (Variables|Default|GetBreakableBomb)) (- (Transformation|GetWorldLocation (Variables|/Game/Level/BombTag/BP_BombBreakable.BP_BombBreakable_C|GetGeometryCollection (Variables|Default|GetBreakableBomb))) "0.000000,0.000000,100.000000") 2e+02 1.5e+04 "RIF_Constant" false)
  (Utilities|Time|SetTimerbyEvent (delegate Custom|Remove%20Broken%20Bits) 4.0)
  (bind _returnvalue_3 (Actor|GetActorOfClass "/Game/Level/BombTag/BP_BombTagManager.BP_BombTagManager_C"))
  (Default|BombExploded _returnvalue_3))

(event Custom|Server%20BombDropped
  (bind _returnvalue (Actor|GetActorOfClass "/Game/Level/BombTag/BP_BombTagManager.BP_BombTagManager_C"))
  (Default|BombDropped _returnvalue))

(event Custom|Server%20UpdateCurrentHolder
  (params (NewParam :type BP%20Third%20Person%20Character%20Object%20Reference))
  (bind _returnvalue (Actor|GetActorOfClass "/Game/Level/BombTag/BP_BombTagManager.BP_BombTagManager_C"))
  (Default|UpdateCurrentHolder _returnvalue NewParam))

(event Custom|Rpc%20LightFuse
  (params (time :type Float%20%28double-precision%29))
  (CallFunction|LightFuse time))

(event Custom|ResetBomb
  (Components|Timeline|SetPlaybackPosition (Variables|Default|GetFuseTimeline) 0.0 true true)
  (Rendering|SetVisibility (Variables|Default|GetStaticMesh) true false)
  (Transformation|SetRelativeLocation (Variables|Default|GetNS_FuseSparks) "0, 0, 0" false false))

(event Custom|Remove%20Broken%20Bits
  (Actor|DestroyActor (Variables|Default|GetBreakableBomb)))

(event EventBeginPlay
  (|CallParentFunction)
  (Variables|Default|SetPiecesCount (Utilities|Array|Length (Components|GetChildrenComponents (Variables|Default|GetBombGC) true)))
  (bind _returnvalue (Actor|GetActorOfClass "/Game/Level/BombTag/BP_BombTagManager.BP_BombTagManager_C"))
  (EventDispatchers|BindEventtoLightBomb _returnvalue (delegate Custom|Rpc%20LightFuse)))

(event EventDropped
  (Transformation|SetActorRotation "0, 0, 0") ; Reset actor rotation to keep hint on top
  (Utilities|FlowControl|Delay 0.2) ; Grace Period to prevent self ragdoll
  (CallFunction|FuncUpdateHeldState false) ; Updates the held state
  (CallFunction|ServerBombDropped))

(fn ConstructionScript
  (|CallParentFunction)
  (bind _returnvalue (Rendering|Material|CreateDynamicMaterialInstance (Variables|Default|GetFuse) 0 "/Game/Art/Meshes/Internal/CustomMeshes/Bomb/FuseMat.FuseMat" "None" :!class /Script/Engine.PrimitiveComponent))
  (Variables|Default|SetFuseDMI _returnvalue)
  (Class|NiagaraComponent|SetSimCache (Variables|Default|GetBombExplosion) "/Game/Art/Meshes/Internal/CustomMeshes/Bomb/NS_Explosion2_SimCache_SimCache_1.NS_Explosion2_SimCache_SimCache_1" false))