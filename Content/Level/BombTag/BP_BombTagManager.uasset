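; Manager for the Bomb Tag mode, running elimination rounds in which the current bomb holder dies on explosion.
; The authority assigns the bomb to a random living player, moves it between players under a transfer cooldown, and returns it after throws.
; Explosions ragdoll and eliminate the holder, then restart the countdown, resetting positions when few players remain, or reload the map via ServerTravel.
; RPC events mirror bomb attachment and HUD text.
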(event Custom|StartGame
  ;[0 1 0] Game Start
  (Networking|SwitchHasAuthority
    (:Authority
      (CallFunction|ServerAddHud)
      (bind _outactors (Actor|GetAllActorsOfClass "/Game/Blueprints/Characters/Goblin/BP_ThirdPersonCharacter.BP_ThirdPersonCharacter_C"))
      (bind _output_get (Variables|Default|SetAlivePlayers _outactors))
      (CallFunction|SetPlayertoSpawn _output_get)
      (bind _returnvalue (Actor|GetActorOfClass "/Game/Level/BombTag/BP_Bomb.BP_Bomb_C"))
      (Variables|Default|SetBomb _returnvalue)
      (Utilities|FlowControl|Delay 0.2)
      (CallFunction|AssignBomb)
      (CallFunction|StartBombTimer))))

(event Custom|AssignBomb
  ;[0 1 0] Bomb Assignment
  (Networking|SwitchHasAuthority
    (:Authority
      (bind _output_get (Variables|Default|SetCurrentBombHolder (.OutItem (Utilities|Array|Random (Variables|Default|GetAlivePlayers)))))
      (CallFunction|ServerUpdateName (Utilities|String|Append "Current Bomb Holder: " (Variables|/Game/Blueprints/Characters/Goblin/BP_ThirdPersonCharacter.BP_ThirdPersonCharacter_C|GetNameStr _output_get)))
      (CallFunction|RPCAssignBomb _output_get)
      (Variables|/Game/Blueprints/Characters/Goblin/BP_ThirdPersonCharacter.BP_ThirdPersonCharacter_C|SetisBombHolder _output_get true)
      (for _array_element (Variables|Default|GetAlivePlayers)
        (if (!= _array_element (Variables|Default|GetCurrentBombHolder))
          (Variables|/Game/Blueprints/Characters/Goblin/BP_ThirdPersonCharacter.BP_ThirdPersonCharacter_C|SetisBombHolder _array_element false))))))

(event Custom|RPC%20UpdateName
  (params (Name :type String))
  ;[0.2462 0.6038 1] HUD
  (Rendering|Components|TextRender|SetText (Variables|/Game/UserInterface/Huds/BombTagHud.BombTagHud_C|GetName (Variables|Default|GetHUD)) (Utilities|Text|ToText(String) Name)))

(event Custom|Server%20UpdateName
  (params (Name :type String))
  ;[0.2462 0.6038 1] HUD
  (CallFunction|RPCUpdateName Name))

(event Custom|StartBombTimer
  ;[0 1 0] Bomb Assignment
  (Default|CallLightBomb (Utilities|NewMacro)))

(event Custom|RPC%20AssignBomb
  (params (Player :type BP%20Third%20Person%20Character%20Object%20Reference))
  ;[0 1 0] Bomb Assignment
  (if (Variables|/Game/Blueprints/Characters/Goblin/BP_ThirdPersonCharacter.BP_ThirdPersonCharacter_C|GetisCarrying Player)
    (Default|FuncDropBox Player) ; Drop any other items the player is holding
  )
  (Utilities|FlowControl|Delay 0.1)
  (Default|FuncAssignBomb Player (Variables|Default|GetBomb)) ; Assign the bomb
)

(event Custom|BombDropped
  ;[0 1 0] Bomb Assignment
  (Utilities|FlowControl|Delay (Variables|Default|GetThrowDuration))
  (CallFunction|RPCAssignBomb (Variables|Default|GetCurrentBombHolder)))

(event Custom|UpdateCurrentHolder
  (params (NewParam :type BP%20Third%20Person%20Character%20Object%20Reference))
  ;[0 1 0] Bomb Assignment
  (if (not (== (Variables|Default|GetCurrentBombHolder) NewParam)) ; Ensure the current bomb holder does NOT equal the cur holder
    (if (<= (Variables|Default|GetBombTransferCooldown) 0.0) ; Wait for cooldown
      (CallFunction|RPCDropBomb (Variables|Default|GetCurrentBombHolder) (Variables|Default|GetBomb))
      (Variables|/Game/Blueprints/Characters/Goblin/BP_ThirdPersonCharacter.BP_ThirdPersonCharacter_C|SetisBombHolder (Variables|Default|GetCurrentBombHolder) false)
      (bind _output_get (Variables|Default|SetCurrentBombHolder NewParam))
      (Variables|/Game/Blueprints/Characters/Goblin/BP_ThirdPersonCharacter.BP_ThirdPersonCharacter_C|SetisBombHolder _output_get true)
      (CallFunction|RPCAssignBomb (Variables|Default|GetCurrentBombHolder))
      (CallFunction|ServerUpdateName (Utilities|String|Append "Current Bomb Holder: " (Variables|/Game/Blueprints/Characters/Goblin/BP_ThirdPersonCharacter.BP_ThirdPersonCharacter_C|GetNameStr (Variables|Default|GetCurrentBombHolder))))
      (Variables|Default|SetBombTransferCooldown (Variables|Default|GetBombTC_Time)))))

(event Custom|BombExploded
  (bind _currentbombholder (Variables|Default|GetCurrentBombHolder))
  (bind _aliveplayers (Variables|Default|GetAlivePlayers))
  (bind _returnvalue (Utilities|Array|Length _aliveplayers))
  ;[0 1 0] Bomb explosion
  (Default|FuncDropBomb _currentbombholder (Variables|Default|GetBomb)) ; Drop the bomb so the player doesnt hold it in the afterlife
  (Default|TriggerRagdoll _currentbombholder true 3.0) ; Ragdoll the player
  (EventDispatchers|BindEventtoDeathEvent _currentbombholder (delegate Custom|ResetActorLoc)) ; Bind an event to player death
  (Utilities|Array|RemoveItem _aliveplayers _currentbombholder) ; Remove the dead player from alive players
  (if (<= _returnvalue 1)
    (CallFunction|ServerUpdateName "WINNER WINNER")
    (Utilities|FlowControl|Delay 0.5)
    (Development|ExecuteConsoleCommand "ServerTravel  /Game/ThirdPerson/Maps/BombTag?listen" 0) ; Restart level
    (else
      (CallFunction|AssignBomb) ; The bomb is reassigned
      (if (<= _returnvalue 3) ; If theplayer coutn is 3 or less
        (CallFunction|SetPlayertoSpawn (Variables|Default|GetAlivePlayers)) ; Return everyone to spawnpoint
        (Default|ResetBomb (Variables|Default|GetBomb)) ; Resest the bomb state
      )
      (CallFunction|StartBombTimer) ; Start the bomb countdown
    )))

(event Custom|ResetActorLoc
  (params (PlayerRef :type BP%20Third%20Person%20Character%20Object%20Reference))
  ;[0 1 0] Bomb explosion
  (Default|ServerUnragdoll PlayerRef 0.0) ; Unragdoll player
  (Utilities|FlowControl|DelayUntilNextTick)
  (Transformation|SetActorLocation PlayerRef "-136040.000000,-31257.000000,-40507.350692" false true) ; Set them to the starting paltform
  (bind _outactors (Actor|GetAllActorsOfClass "/Game/Blueprints/Systems/Chat/BP_GamePC.BP_GamePC_C")) ; Get all players
  (for _array_element _outactors
    (Default|MulticastSystemMessage (Actor|GetComponentbyClass _array_element "/Game/Blueprints/Systems/Chat/AC_ChatPC.AC_ChatPC_C") (Utilities|String|Append (PlayerState|GetPlayerName (Variables|/Script/Engine.Pawn|GetPlayerState PlayerRef)) " exploded!") "(R=0.000000,G=0.000000,B=0.000000,A=1.000000)") ; Broadcast the message to all players
  ))

(event Custom|RPC%20DropBomb
  (params (RpcBombHolder :type BP%20Third%20Person%20Character%20Object%20Reference) (Bomb :type BP%20Bomb%20Object%20Reference))
  ;[0 1 0] Bomb Assignment
  (Default|FuncDropBomb RpcBombHolder Bomb))

(event Custom|Server%20Add%20Hud
  ;[0.2462 0.6038 1] HUD
  (CallFunction|RPCAddHud))

(event Custom|RPC%20Add%20Hud
  ;[0.2462 0.6038 1] HUD
  (bind _returnvalue (UserInterface|CreateWidget "/Game/UserInterface/Huds/BombTagHud.BombTagHud_C"))
  (Variables|Default|SetHUD _returnvalue)
  (UserInterface|Viewport|AddtoViewport _returnvalue 0))

(event EventTick
  (params (DeltaSeconds :type Float%20%28single-precision%29))
  ;[0 1 0] EventTick
  (Networking|SwitchHasAuthority
    (:Authority
      (Variables|Default|SetBombTransferCooldown (Math|Float|Clamp(Float) (- (Variables|Default|GetBombTransferCooldown) DeltaSeconds) 0.0 1e+02))
      (for _array_element (Variables|Default|GetAlivePlayers)
        (if (or (Variables|/Game/Blueprints/Characters/Goblin/BP_ThirdPersonCharacter.BP_ThirdPersonCharacter_C|GetisDead _array_element) (not (Utilities|IsValid _array_element)))
          (Utilities|Array|RemoveItem (Variables|Default|GetAlivePlayers) _array_element))
        (if (and (!= (Variables|Default|GetCurrentBombHolder) _array_element) (== (Variables|/Game/Blueprints/Characters/Goblin/BP_ThirdPersonCharacter.BP_ThirdPersonCharacter_C|GetCurrentBox _array_element) (Variables|Default|GetBomb)))
          (Variables|/Game/Blueprints/Characters/Goblin/BP_ThirdPersonCharacter.BP_ThirdPersonCharacter_C|SetCurrentBox _array_element 0))))))

(fn ConstructionScript)

(fn BombHolder
  (params (NewParam1 :type BP%20Third%20Person%20Character%20Object%20Reference))
  (return false))

(fn SetPlayertoSpawn
  (params (Array :type Array%20of%20BP%20Third%20Person%20Character%20Object%20References))
  (for _array_element Array
    (Transformation|SetActorLocation _array_element "-137660.000374,-28889.998327,-45380.000000" false true)))