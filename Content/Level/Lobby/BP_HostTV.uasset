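; Lobby TV that only the host can interact with, hosting the HostTV menu widget and relaying the lobby code to a painting's text.
; Sphere overlap shows a key hint that turns toward the player camera and binds the character's interact event.
; Interacting toggles focus by blending the view to the TV, enabling UI input and cursor, and disabling movement.
; Code updates pass through RPCUpdateLobbyCode, which remote instances also call on BeginPlay.
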(event OnComponentBeginOverlap(Sphere)
  (params (OverlappedComponent :type Primitive%20Component%20Object%20Reference) (OtherActor :type Actor%20Object%20Reference) (OtherComp :type Primitive%20Component%20Object%20Reference) (OtherBodyIndex :type Integer) (bFromSweep :type Boolean) (SweepResult :type Hit%20Result%20Structure%20%28by%20ref%29))
  ;[0.2462 0.6038 1] Widget Handling
  (bind _asbp_third_person_character (Utilities|Casting|CastToBP_ThirdPersonCharacter OtherActor))
  (if (Ability|HasAuthority (Game|GetPlayerController 0))
    (bind _asbp_third_person_character_2 (Utilities|Casting|CastToBP_ThirdPersonCharacter (Game|GetPlayerCharacter 0)))
    (Development|SetHiddeninGame (Variables|Default|GetWidget1) false false)
    (Variables|Default|SetPlayerInSphere true)
    (EventDispatchers|BindEventtoInteractEvent _asbp_third_person_character (delegate Custom|HostTv))
    (bind _aswdp_key_hint_1 (Utilities|Casting|CastToWDP_KeyHint1 (UserInterface|GetWidget (Variables|Default|GetWidget1))))
    (Default|UpdateKey _aswdp_key_hint_1)))

(event OnComponentEndOverlap(Sphere)
  (params (OverlappedComponent :type Primitive%20Component%20Object%20Reference) (OtherActor :type Actor%20Object%20Reference) (OtherComp :type Primitive%20Component%20Object%20Reference) (OtherBodyIndex :type Integer))
  ;[0.2462 0.6038 1] Widget Handling
  (bind _asbp_third_person_character (Utilities|Casting|CastToBP_ThirdPersonCharacter OtherActor))
  (if (Ability|HasAuthority (Game|GetPlayerController 0))
    (Development|SetHiddeninGame (Variables|Default|GetWidget1) true false)
    (Variables|Default|SetPlayerInSphere false)
    (if (Utilities|IsValid _asbp_third_person_character)
      (EventDispatchers|UnbindallEventsfromInteractEvent _asbp_third_person_character))))

(event Custom|HostTv
  (params (Host :type Boolean))
  ;[0.2462 0.6038 1] Widget Handling
  ;;[1 0.01298 0.9047] Interaction
  (CallFunction|FuncInteractwithDevice Host))

(event Custom|UpdateLobbyCode
  (params (Code :type String))
  (bind _output_get (Variables|Default|SetLobbyCode Code))
  (CallFunction|RPCUpdateLobbyCode _output_get))

(event Custom|RPC%20UpdateLobbyCode
  (params (code :type String))
  (bind _lobbycodepainting (Variables|Default|GetLobbyCodePainting))
  (Utilities|IsValid _lobbycodepainting
    (:Is%20Valid
      (Rendering|Components|TextRender|SetText (Variables|/Script/Engine.TextRenderActor|GetTextRender _lobbycodepainting) (Utilities|Text|ToText(String) code)))))

(event Custom|RefreshCode
  (CallFunction|RPCUpdateLobbyCode (stale Custom|UpdateLobbyCode _output_get)))

(event EventBeginPlay
  (Networking|SwitchHasAuthority
    (:Authority
      _)
    (:Remote
      (CallFunction|RefreshCode)))
  (bind _ashost_tv (Utilities|Casting|CastToHostTV (UserInterface|GetWidget (Variables|Default|GetWidget))))
  (Variables|/Game/UserInterface/Menus/HostTV.HostTV_C|SetHostTV _ashost_tv self)
  ;[0.2462 0.6038 1] Widget Handling
  (Development|SetHiddeninGame (Variables|Default|GetWidget1) true false)
  (Variables|Default|SetPlayerInSphere false)
  (if (Utilities|IsValid (stale OnComponentEndOverlap(Sphere) _asbp_third_person_character))
    (EventDispatchers|UnbindallEventsfromInteractEvent (stale OnComponentEndOverlap(Sphere) _asbp_third_person_character))))

(event Collision|EventActorBeginOverlap
  (params (OtherActor :type Actor%20Object%20Reference)))

(event EventTick
  (params (DeltaSeconds :type Float%20%28single-precision%29))
  (bind _widget1 (Variables|Default|GetWidget1))
  ;[0.2462 0.6038 1] Widget Handling
  (if (and (Variables|Default|GetPlayerInSphere) (Utilities|IsValid (stale OnComponentBeginOverlap(Sphere) _asbp_third_person_character_2)))
    (Transformation|SetWorldRotation _widget1 (Math|Rotator|FindLookatRotation (Transformation|GetWorldLocation _widget1) (Transformation|GetWorldLocation (Variables|/Script/RoomOne.RoomOneCharacter|GetFollowCamera (stale OnComponentBeginOverlap(Sphere) _asbp_third_person_character_2)))) false false)))

(fn ConstructionScript)

(fn FuncInteractwithDevice
  (params (Condition :type Boolean))
  (bind _returnvalue (Game|GetPlayerCharacter 0))
  (bind _returnvalue_2 (Game|GetPlayerController 0))
  (bind _widget1 (Variables|Default|GetWidget1))
  (bind _charactermovement (Variables|/Script/Engine.Character|GetCharacterMovement _returnvalue))
  (if Condition
    (if (Variables|Default|GetisFocused)
      (Game|Player|SetViewTargetwithBlend _returnvalue_2 _returnvalue 0.0 "VTBlend_Linear" 0.0 false)
      (Input|SetInputModeGameOnly _returnvalue_2 false)
      (Variables|/Script/Engine.PlayerController|SetbShowMouseCursor _returnvalue_2 false)
      (Pawn|Components|CharacterMovement|SetMovementMode _charactermovement "MOVE_Walking" 0)
      (Development|SetHiddeninGame _widget1 false false)
      (Variables|Default|SetisFocused false)
      (else
        (Game|Player|SetViewTargetwithBlend _returnvalue_2 self 0.0 "VTBlend_Linear" 0.0 false)
        (Input|SetInputModeGameandUI _returnvalue_2 0 "DoNotLock" false false)
        (Variables|/Script/Engine.PlayerController|SetbShowMouseCursor _returnvalue_2 true)
        (Pawn|Components|CharacterMovement|DisableMovement _charactermovement)
        (Development|SetHiddeninGame _widget1 true false)
        (Variables|Default|SetisFocused true)))))