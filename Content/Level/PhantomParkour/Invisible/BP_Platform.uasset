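; BP_Platform is an invisible platform in the Phantom Parkour level that reveals itself when the player touches it.
; On BeginPlay it hides itself in game and gives its mesh a dynamic material instance with a random dark PlatformColor.
; When BP_ThirdPersonCharacter overlaps its Box trigger, it unhides and plays a bell sound at its location, with no logic to hide it again.
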(event OnComponentBeginOverlap(Box)
  (params (OverlappedComponent :type Primitive%20Component%20Object%20Reference) (OtherActor :type Actor%20Object%20Reference) (OtherComp :type Primitive%20Component%20Object%20Reference) (OtherBodyIndex :type Integer) (bFromSweep :type Boolean) (SweepResult :type Hit%20Result%20Structure%20%28by%20ref%29))
  ;[0.15 0.15 0.15 0.5] Unhide Actor and Play Sound on collision with Platform
  (Utilities|Casting|CastToBP_ThirdPersonCharacter OtherActor)
  (Rendering|SetActorHiddenInGame false)
  (Audio|PlaySoundatLocation "/Game/Level/PhantomParkour/Invisible/gPentBell1_Cue_COPY.gPentBell1_Cue_COPY" (Transformation|GetActorLocation) "0, 0, 0" 1.0 1.0 0.0 0 0 0 0))

(event EventBeginPlay
  ;[0.15 0.15 0.15 0.5] Set Random Material Colour
  (Rendering|SetActorHiddenInGame true)
  (bind _returnvalue (Rendering|Material|CreateDynamicMaterialInstance (Variables|Default|GetStatic%20Mesh) 0 "/Game/Level/PhantomParkour/Invisible/M_PlatformColor.M_PlatformColor" "None" :!class /Script/Engine.PrimitiveComponent))
  (Rendering|Material|SetMaterial (Variables|Default|GetStatic%20Mesh) 0 _returnvalue)
  (bind _output_get (Variables|Default|SetDynamicMaterial _returnvalue))
  (Rendering|Material|SetVectorParameterValue _output_get "PlatformColor" (Utilities|Struct|MakeLinearColor (Math|Random|RandomFloatinRange 0.0 0.4) (Math|Random|RandomFloatinRange 0.0 0.4) (Math|Random|RandomFloatinRange 0.0 0.4) 0.0) :!class /Script/Engine.MaterialInstanceDynamic))

(fn ConstructionScript)