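; Child Blueprint of a checkpoint stairs actor in the RopedTogether level that raises its stairs when ActivateStairsAll fires.
; A Timeline lerps the Stairs component's relative location upward along Z, without sweep.
; Each Timeline update activates the Audio component, whose active state also gates the event against retriggering while it plays.
; Construction defers to the parent script.
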(event EventBeginPlay)

(event Collision|EventActorBeginOverlap
  (params (OtherActor :type Actor%20Object%20Reference)))

(event EventTick
  (params (DeltaSeconds :type Float%20%28single-precision%29)))

(event EventActivateStairsAll
  (if (not (Components|Activation|IsActive (Variables|Default|GetAudio)))
    (bind _alpha (Timeline|Timeline Play)
      (:Update
        (Transformation|SetRelativeLocation (Variables|Default|GetStairs) (Math|Vector|Lerp(Vector) "0, 0, 0" "0.000000,0.000000,800.000000" _alpha) false false)
        (Components|Activation|Activate (Variables|Default|GetAudio) false)))))

(fn ConstructionScript
  (|CallParentFunction))