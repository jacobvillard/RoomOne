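; BP_ConveyorBelt is a conveyor belt level actor that carries player characters along its surface.
; Each Tick it offsets every BP_ThirdPersonCharacter overlapping its Box along the Arrow's forward vector by Speed times delta time, without sweeping.
; The Construction Script gives the mesh a dynamic chevron material whose Y scroll rate is derived from the same Speed, tying the visual to the push.
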(event EventTick
  (params (DeltaSeconds :type Float%20%28single-precision%29))
  (for _array_element (Collision|GetOverlappingActors (Variables|Default|GetBox) "/Game/Blueprints/Characters/Goblin/BP_ThirdPersonCharacter.BP_ThirdPersonCharacter_C" :!class /Script/Engine.PrimitiveComponent)
    (Transformation|AddActorWorldOffset _array_element (* (* DeltaSeconds (Variables|Default|GetSpeed)) (Math|Vector|GetForwardVector (Transformation|GetWorldRotation (Variables|Default|GetArrow)))))))

(fn ConstructionScript
  (bind _returnvalue (Rendering|Material|CreateDynamicMaterialInstance (Variables|Default|GetStaticMesh) 0 "/Game/Art/Materials/ChevronPattern_Mat.ChevronPattern_Mat" "None" :!class /Script/Engine.PrimitiveComponent))
  (bind _output_get (Variables|Default|SetDMI _returnvalue))
  (Rendering|Material|SetScalarParameterValue _output_get "CoordinateX" 1e+01 :!class /Script/Engine.MaterialInstanceDynamic)
  (Rendering|Material|SetScalarParameterValue _output_get "CoordinateY" 1e+01 :!class /Script/Engine.MaterialInstanceDynamic)
  (Rendering|Material|SetScalarParameterValue _output_get "SpeedX" 0.0 :!class /Script/Engine.MaterialInstanceDynamic)
  (Rendering|Material|SetScalarParameterValue _output_get "SpeedY" (/ (Variables|Default|GetSpeed) 1.2e+03) :!class /Script/Engine.MaterialInstanceDynamic)
  (Rendering|Material|SetMaterial (Variables|Default|GetStaticMesh) 0 _output_get))