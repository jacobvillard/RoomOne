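; Elevator actor that carries a scene component between its base and a configurable height, with sliding double doors and travel audio.
; Overlapping the Box binds the character's interact event to closing the doors, while a second box opens them on first overlap only.
; Two timelines chain the cycle: doors finishing closing start travel up or down by ElevatorAtTop, and arrival reopens them.
; Construction script applies PlayRate to the travel timeline.
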(event OnComponentBeginOverlap(Box)
  (params (OverlappedComponent :type Primitive%20Component%20Object%20Reference) (OtherActor :type Actor%20Object%20Reference) (OtherComp :type Primitive%20Component%20Object%20Reference) (OtherBodyIndex :type Integer) (bFromSweep :type Boolean) (SweepResult :type Hit%20Result%20Structure%20%28by%20ref%29))
  (bind _asbp_third_person_character (Utilities|Casting|CastToBP_ThirdPersonCharacter OtherActor))
  (EventDispatchers|BindEventtoInteractEvent _asbp_third_person_character (delegate Custom|MoveElevator)))

(event OnComponentBeginOverlap(OpenDoorBox)
  (params (OverlappedComponent :type Primitive%20Component%20Object%20Reference) (OtherActor :type Actor%20Object%20Reference) (OtherComp :type Primitive%20Component%20Object%20Reference) (OtherBodyIndex :type Integer) (bFromSweep :type Boolean) (SweepResult :type Hit%20Result%20Structure%20%28by%20ref%29))
  (Utilities|Casting|CastToBP_ThirdPersonCharacter OtherActor)
  (Utilities|FlowControl|DoOnce false
    (:Completed
      (CallFunction|ServerOpenDoors))))

(event Custom|MoveElevator
  (params (Host :type Boolean))
  (CallFunction|ServerCloseDoors))

(event Custom|Elevator%20Up
  (Components|Activation|Activate (Variables|Default|GetAudio) true)
  (bind (_direction _go_) (Timeline|Elevator Play)
    (:Update
      (Transformation|SetRelativeLocation (Variables|Default|GetScene) (Math|Vector|MakeVector 0.0 0.0 (Math|Float|Lerp 0.0 (Variables|Default|GetDistanceUp) _go_)) false false))
    (:Finished
      (CallFunction|OpenDoors)
      (switch Utilities|FlowControl|Switch|SwitchonETimelineDirection _direction
        (:Forward
          (Variables|Default|SetElevatorAtTop true))
        (:Backward
          (Variables|Default|SetElevatorAtTop false))))))

(event Custom|Elevator%20Down
  (Components|Activation|Activate (Variables|Default|GetAudio) true)
  (bind (_direction _go_) (Timeline|Elevator Reverse)
    (:Update
      (Transformation|SetRelativeLocation (Variables|Default|GetScene) (Math|Vector|MakeVector 0.0 0.0 (Math|Float|Lerp 0.0 (Variables|Default|GetDistanceUp) _go_)) false false))
    (:Finished
      (CallFunction|OpenDoors)
      (switch Utilities|FlowControl|Switch|SwitchonETimelineDirection _direction
        (:Forward
          (Variables|Default|SetElevatorAtTop true))
        (:Backward
          (Variables|Default|SetElevatorAtTop false))))))

(event Custom|CloseDoors
  (Components|Activation|Deactivate (Variables|Default|GetAudio))
  (bind (_direction _dooralpha) (Timeline|Doors Reverse)
    (:Update
      (Transformation|SetRelativeLocation (Variables|Default|GetDoorRight) (Math|Vector|MakeVector (Math|Float|Lerp 0.0 (Variables|Default|GetDoorDistance) _dooralpha) 0.0 0.0) false false)
      (Transformation|SetRelativeLocation (Variables|Default|GetDoorLeft) (Math|Vector|MakeVector (* (Math|Float|Lerp 0.0 (Variables|Default|GetDoorDistance) _dooralpha) -1.0) 0.0 0.0) false false)
      (Variables|Default|SetCanMove false))
    (:Finished
      (switch Utilities|FlowControl|Switch|SwitchonETimelineDirection _direction
        (:Backward
          (if (Variables|Default|GetElevatorAtTop)
            (CallFunction|ElevatorDown)
            (else
              (CallFunction|ElevatorUp))))))))

(event Custom|OpenDoors
  (Components|Activation|Deactivate (Variables|Default|GetAudio))
  (bind (_direction _dooralpha) (Timeline|Doors Play)
    (:Update
      (Transformation|SetRelativeLocation (Variables|Default|GetDoorRight) (Math|Vector|MakeVector (Math|Float|Lerp 0.0 (Variables|Default|GetDoorDistance) _dooralpha) 0.0 0.0) false false)
      (Transformation|SetRelativeLocation (Variables|Default|GetDoorLeft) (Math|Vector|MakeVector (* (Math|Float|Lerp 0.0 (Variables|Default|GetDoorDistance) _dooralpha) -1.0) 0.0 0.0) false false)
      (Variables|Default|SetCanMove false))
    (:Finished
      (switch Utilities|FlowControl|Switch|SwitchonETimelineDirection _direction
        (:Backward
          (if (Variables|Default|GetElevatorAtTop)
            (CallFunction|ElevatorDown)
            (else
              (CallFunction|ElevatorUp))))))))

(event Custom|ServerCloseDoors
  (CallFunction|CloseDoors))

(event Custom|ServerOpenDoors
  (CallFunction|OpenDoors))

(fn ConstructionScript
  (Components|Timeline|SetPlayRate (Variables|Default|GetElevator) (Variables|Default|GetPlayRate)))