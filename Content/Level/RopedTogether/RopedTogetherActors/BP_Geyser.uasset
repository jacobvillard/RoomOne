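; BP_Geyser is a level obstacle that toggles on and off and launches player characters upward while active.
; It binds to the RopeActivator's activate-all-moving-obstacles event, which starts a looping timer.
; Each tick of that timer flips the active state through a multicast event, switching particle velocity and the Blast component.
; A capsule overlap during the active state calls a server event that applies LaunchCharacter to the third-person character.
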(event OnComponentBeginOverlap(Capsule)
  (params (OverlappedComponent :type Primitive%20Component%20Object%20Reference) (OtherActor :type Actor%20Object%20Reference) (OtherComp :type Primitive%20Component%20Object%20Reference) (OtherBodyIndex :type Integer) (bFromSweep :type Boolean) (SweepResult :type Hit%20Result%20Structure%20%28by%20ref%29))
  (if (Variables|Default|GetGeyserActive)
    (bind _asbp_third_person_character (Utilities|Casting|CastToBP_ThirdPersonCharacter OtherActor))
    (CallFunction|ServerLaunchPlayer _asbp_third_person_character)))

(event Custom|Activate
  (Utilities|Time|SetTimerbyEvent (delegate Custom|GeyserToggle) (Variables|Default|GetGeyserTime) true false 0.2))

(event Custom|GeyserToggle
  (CallFunction|TriggerGeyser))

(event Custom|Multicast%20Geyser
  (bind _geyserparticles (Variables|Default|GetGeyserParticles))
  (bind _output_get (Variables|Default|SetGeyserActive (not (Variables|Default|GetGeyserActive))))
  (if _output_get
    (Niagara|SetNiagaraVariable(Float) _geyserparticles "Velocity" (Variables|Default|GetHighEmit))
    (Components|Activation|Activate (Variables|Default|GetBlast) true)
    (else
      (Niagara|SetNiagaraVariable(Float) _geyserparticles "Velocity" (Variables|Default|GetLowEmit))
      (Components|Activation|Deactivate (Variables|Default|GetBlast)))))

(event Custom|TriggerGeyser
  (CallFunction|MulticastGeyser))

(event Custom|ServerLaunchPlayer
  (params (Player :type BP%20Third%20Person%20Character%20Object%20Reference))
  (Character|LaunchCharacter Player (Math|Vector|MakeVector 0.0 0.0 (Variables|Default|GetLaunchVelocity)) true true))

(event EventBeginPlay
  (bind _returnvalue (Actor|GetActorOfClass "/Game/Level/RopedTogether/RopedTogetherActors/RopeActivator.RopeActivator_C"))
  (EventDispatchers|BindEventtoActivateAllMovingObstacles _returnvalue (delegate Custom|Activate))
  (Niagara|SetNiagaraVariable(Float) (Variables|Default|GetGeyserParticles) "Velocity" (Variables|Default|GetHighEmit)))

(fn ConstructionScript)