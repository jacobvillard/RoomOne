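; Swinging pendulum obstacle that knocks third-person characters it hits, starting after a time offset once the RopeActivator signals all moving obstacles.
; A timeline ping-pongs the pivot between mirrored max angles, activating audio near mid-swing.
; A looping timer derives the sphere's velocity from position deltas, and overlaps launch the character with that velocity scaled by hit strength.
; The construction script sets ball height, swing limits and play rate.
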(event OnComponentBeginOverlap(Sphere)
  (params (OverlappedComponent :type Primitive%20Component%20Object%20Reference) (OtherActor :type Actor%20Object%20Reference) (OtherComp :type Primitive%20Component%20Object%20Reference) (OtherBodyIndex :type Integer) (bFromSweep :type Boolean) (SweepResult :type Hit%20Result%20Structure%20%28by%20ref%29))
  (bind _asbp_third_person_character (Utilities|Casting|CastToBP_ThirdPersonCharacter OtherActor))
  (CallFunction|ServerLaunchPlayer _asbp_third_person_character))

(event Custom|TriggerPendulum
  (params (Forward? :type Boolean))
  (if Forward?
    (bind _swing (Timeline|Swinging Play)
      (:Update
        (Transformation|SetRelativeRotation (Variables|Default|GetPivot) (Math|Rotator|Lerp(Rotator) (Variables|Default|GetStartingRot) (Variables|Default|GetEndingRot) _swing) false true)
        (if (Math|Float|InRange(Float) _swing 0.45 0.55 false false)
          (Components|Activation|Activate (Variables|Default|GetAudio) true)))
      (:Finished
        (CallFunction|TriggerPendulum (not Forward?))))
    (else
      (Timeline|Swinging Reverse))))

(event Custom|CalculateSphereVelocity
  (bind _output_get (Variables|Default|SetNewLoc (Transformation|GetWorldLocation (Variables|Default|GetSphere))))
  (Variables|Default|SetVelocity (/ (- _output_get (Variables|Default|GetOldLoc)) (Variables|Default|GetDeltaTime)))
  (Variables|Default|SetOldLoc (Variables|Default|GetNewLoc)))

(event Custom|Activate
  (Utilities|FlowControl|Delay (Variables|Settings|GetTimeOffset))
  (CallFunction|TriggerPendulum true)
  (Variables|Default|SetOldLoc (Transformation|GetWorldLocation (Variables|Default|GetSphere)))
  (Utilities|Time|SetTimerbyFunctionName 0 "CalculateSphereVelocity" (Variables|Default|GetDeltaTime) true))

(event Custom|ServerLaunchPlayer
  (params (Player :type BP%20Third%20Person%20Character%20Object%20Reference))
  (Character|LaunchCharacter Player (* (Variables|Default|GetVelocity) (Variables|Settings|GetHitStrength)) false false))

(event EventBeginPlay
  (bind _returnvalue (Actor|GetActorOfClass "/Game/Level/RopedTogether/RopedTogetherActors/RopeActivator.RopeActivator_C"))
  (EventDispatchers|BindEventtoActivateAllMovingObstacles _returnvalue (delegate Custom|Activate)))

(fn ConstructionScript
  (bind _maxangle (Variables|Settings|GetMaxAngle))
  (Components|Timeline|SetPlaybackPosition (Variables|Default|GetSwinging) 0.5 false true)
  (Transformation|SetRelativeLocation (Variables|Default|GetStaticMesh) (Math|Vector|MakeVector 0.0 0.0 (Variables|Settings|GetBallHeight)) false false)
  (Variables|Default|SetStartingRot (Math|Rotator|MakeRotator 0.0 (* _maxangle -1.0) 0.0))
  (Variables|Default|SetEndingRot (Math|Rotator|MakeRotator 0.0 _maxangle 0.0))
  (Components|Timeline|SetPlayRate (Variables|Default|GetSwinging) (/ 1.0 (Variables|Settings|GetTimePerSwing))))