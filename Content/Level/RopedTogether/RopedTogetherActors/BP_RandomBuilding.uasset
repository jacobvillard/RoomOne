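; BP_RandomBuilding is a building actor for the RopedTogether level that varies its own look through a Randomise function.
; Randomise picks a random mesh from the Meshes array, applies a dynamic instance of the Building material with a random Darken value, and sets an independent random world scale on each axis.
; The construction script is empty, and nothing in this file calls Randomise.
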(fn ConstructionScript)

(fn Randomise
  (Components|StaticMesh|SetStaticMesh (Variables|Default|GetStaticMesh) (.OutItem (Utilities|Array|Random (Variables|Default|GetMeshes))))
  (bind _returnvalue (Rendering|Material|CreateDynamicMaterialInstance (Variables|Default|GetStaticMesh) 0 "/Game/Art/Meshes/Internal/CustomMeshes/City/Building.Building" "None" :!class /Script/Engine.PrimitiveComponent))
  (Audio|Parameter|SetFloatParameter _returnvalue "Darken" (Math|Random|RandomFloatinRange 0.005 0.3) :!class /Script/AudioExtensions.AudioParameterControllerInterface)
  (Transformation|SetWorldScale3D (Variables|Default|GetStaticMesh) (Math|Vector|MakeVector (Math|Random|RandomFloatinRange 0.5 2.0) (Math|Random|RandomFloatinRange 0.5 2.0) (Math|Random|RandomFloatinRange 0.5 2.0))))