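; Spinning platform obstacle that starts rotating when the level's RopeActivator broadcasts its activate-all-moving-obstacles event.
; A timeline, rate-scaled by TimeFor360, lerps the mesh's relative rotation through a full turn, playing forward or in reverse according to Clockwise.
; Each finished timeline re-triggers activation through the RPC event to keep the spin looping, and audio activates around the half-turn mark.
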(event Custom|Activate
  (CallFunction|RPC))

(event Custom|RPC
  (if (Variables|Settings|GetClockwise)
    (bind _alpha (Timeline|SpinningPlatform PlayFromStart)
      (:Update
        (Transformation|SetRelativeRotation (Variables|Default|GetStaticMesh) (Math|Rotator|Lerp(Rotator) "0, 0, 0" "0.000000,360.000000,0.000000" _alpha) false false)
        (if (Math|Float|InRange(Float) _alpha 0.47 0.53 false false)
          (Components|Activation|Activate (Variables|Default|GetAudio) true)))
      (:Finished
        (CallFunction|Activate)))
    (else
      (Timeline|SpinningPlatform ReverseFromEnd))))

(event EventBeginPlay
  (Components|Timeline|SetPlayRate (Variables|Default|GetSpinningPlatform) (/ 1.0 (Variables|Settings|GetTimeFor360)))
  (bind _returnvalue (Actor|GetActorOfClass "/Game/Level/RopedTogether/RopedTogetherActors/RopeActivator.RopeActivator_C"))
  (EventDispatchers|BindEventtoActivateAllMovingObstacles _returnvalue (delegate Custom|Activate)))

(fn ConstructionScript)