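; SoundBP is an actor that plays looping-timer-driven audio feedback, pairing a sound with a point light that responds to player distance.
; On BeginPlay it starts the audio and a repeating timer that brightens the light as the player nears.
; The same timer line-traces to the player to fake occlusion, cutting volume to a distance-scaled quarter or less when blocked and restoring full volume otherwise.
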(event Custom|AudioFeedback
  (bind _returnvalue (Game|GetPlayerCharacter 0))
  (bind _self self)
  (bind _returnvalue_2 (Transformation|GetDistanceTo _returnvalue _self))
  ;[0.15 0.15 0.15 0.5] Set Intensity
  (Rendering|Components|Light|SetIntensity (Variables|Default|GetPointLight) (Math|Float|MapRangeClamped _returnvalue_2 0.0 1.5e+03 5e+04 0.0))
  ;[0.15 0.15 0.15 0.5] Sound Muffling
  (bind _outhit (Collision|LineTraceByChannel (Transformation|GetActorLocation) (Transformation|GetActorLocation (Game|GetPlayerCharacter 0)) "TraceTypeQuery1" false 0 "None"))
  (if (.bBlockingHit (Collision|BreakHitResult _outhit))
    (Variables|Default|SetVolume%20Multiplier (/ (Math|Float|MapRangeClamped _returnvalue_2 0.0 1e+04 1.0 0.0) 4.0))
    (else
      (bind _output_get (Variables|Default|SetVolume%20Multiplier 1.0))))
  (Audio|Components|Audio|SetVolumeMultiplier (Variables|Default|GetAudio) _output_get :!class /Script/Engine.AudioComponent))

(event EventBeginPlay
  ;[0.15 0.15 0.15 0.5] Play Sound
  (Audio|Components|Audio|Play (Variables|Default|GetAudio) 0.0)
  (Utilities|Time|SetTimerbyEvent (delegate Custom|AudioFeedback) 0.1 true))

(fn ConstructionScript)